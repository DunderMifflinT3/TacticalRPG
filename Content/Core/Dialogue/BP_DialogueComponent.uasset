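; Dialogue component that looks up conversation lines in the DT_TestDialogue data table, apparently an early skeleton.
; InitiateDialogue picks the opening row from the InitiationDialogue map by initiator, falling back to "Default", and removes the used entry so each opener fires once.
; ContinueDialogue fetches the row for the given line number, with 0 routing to EndDialogue.
; Fetched rows are not yet used, and EndDialogue is empty.
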(event Custom|InitiateDialogue
  (params (Initiator :type Text))
  (bind _returnvalue (Utilities|String|ToString(Text) Initiator))
  (bind _initiationdialogue (Variables|Default|GetInitiationDialogue))
  (bind (_value _returnvalue_2) (Utilities|Map|Find _initiationdialogue _returnvalue))
  (if _returnvalue_2
    (Utilities|GetDataTableRow "/Game/Core/Dialogue/DT_TestDialogue.DT_TestDialogue" (Utilities|String|StringToName (Utilities|String|ToString(Integer) _value))
      (:then
        (Utilities|Map|Remove (Variables|Default|GetInitiationDialogue) _returnvalue)))
    (else
      (Utilities|GetDataTableRow "/Game/Core/Dialogue/DT_TestDialogue.DT_TestDialogue" (Utilities|String|StringToName (Utilities|String|ToString(Integer) (.Value (Utilities|Map|Find (Variables|Default|GetInitiationDialogue) "Default"))))
        (:then
          (Utilities|Map|Remove (Variables|Default|GetInitiationDialogue) "Default"))))))

(event Custom|EndDialogue)

(event Custom|ContinueDialogue
  (params (NextLine :type Integer))
  (if (!= NextLine 0)
    (Utilities|GetDataTableRow "/Game/Core/Dialogue/DT_TestDialogue.DT_TestDialogue" (Utilities|String|StringToName (Utilities|String|ToString(Integer) NextLine)))
    (else
      (CallFunction|EndDialogue))))