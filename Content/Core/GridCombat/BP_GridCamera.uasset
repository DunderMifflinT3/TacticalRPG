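; BP_GridCamera is the grid combat camera actor, handling panning, zooming and unit following.
; Construction finds BP_GridManager and derives XY pan bounds from its grid size and tile size.
; Manual panning scales with spring arm length, clamps to those bounds and eases height toward a camera-to-root visibility trace hit.
; PanToActor uses a timeline lerp, Tick snaps to any valid FollowActor when that pan isn't running, and zoom adjusts clamped arm length.
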(event Custom|Set%20Up%20Camera
  (Game|Player|SetViewTargetwithBlend (Game|GetPlayerController 0) self 0.0 "VTBlend_Linear" 0.0 false))

(event Custom|PanToActor
  (params (Actor :type Actor%20Object%20Reference))
  (Variables|Default|SetbPanning true)
  (bind _progress (Timeline|TL_PanToUnit PlayFromStart)
    (:Update
      (Transformation|SetActorLocation (Math|Vector|Lerp(Vector) (Transformation|GetActorLocation) (Transformation|GetActorLocation Actor) _progress) false false))
    (:Finished
      (Variables|Default|SetbPanning false))))

(event Custom|PanCamera
  (params (X :type Float%20%28single-precision%29) (Y :type Float%20%28single-precision%29))
  (bind _returnvalue (Transformation|GetActorLocation))
  (bind _maxcamerabounds (Variables|Default|GetMaxCameraBounds))
  (bind _panspeed (Variables|Default|GetPanSpeed))
  (bind _springarm (Variables|Default|GetSpringArm))
  (bind _defaultsceneroot (Variables|Default|GetDefaultSceneRoot))
  (bind _mincamerabounds (Variables|Default|GetMinCameraBounds))
  (bind _returnvalue_2 (Transformation|GetWorldLocation _defaultsceneroot))
  (bind _targetarmlength (Variables|/Script/Engine.SpringArmComponent|GetTargetArmLength _springarm))
  (bind _returnvalue_3 (* _targetarmlength _panspeed))
  (if (Variables|Default|GetbCanPan)
    ;[1 1 1] Traces to find height difference where the camera is pointing
    (bind _outhit (Collision|LineTraceByChannel (Transformation|GetWorldLocation (Variables|Default|GetCamera)) _returnvalue_2 "TraceTypeQuery1" false 0 "None"))
    (Transformation|SetActorLocation (Math|Vector|MakeVector (Math|Float|Clamp(Float) (+ (.x _returnvalue) (* X _returnvalue_3)) (.x _mincamerabounds) (.x _maxcamerabounds)) (Math|Float|Clamp(Float) (+ (.y _returnvalue) (* Y _returnvalue_3)) (.y _mincamerabounds) (.y _maxcamerabounds)) (Math|Interpolation|FInterpTo (.Z (Math|Vector|BreakVector _returnvalue_2)) (.z (.location _outhit)) 0.005 8.0)) false false)))

(event Custom|ZoomCamera
  (params (Amount :type Float%20%28single-precision%29))
  (Variables|/Script/Engine.SpringArmComponent|SetTargetArmLength (Variables|Default|GetSpringArm) (Math|Float|Clamp(Float) (Math|Interpolation|FInterpTo (Variables|/Script/Engine.SpringArmComponent|GetTargetArmLength (Variables|Default|GetSpringArm)) (+ (Variables|/Script/Engine.SpringArmComponent|GetTargetArmLength (Variables|Default|GetSpringArm)) (* Amount (Variables|Default|GetZoomSpeed))) 1.0 8.0) (Variables|Default|GetMinZoom) (Variables|Default|GetMaxZoom))))

(event EventTick
  (params (DeltaSeconds :type Float%20%28single-precision%29))
  (bind _followactor (Variables|Default|GetFollowActor))
  ;[1 1 1] Follows the active unit after panning to them
  (if (and (not (Variables|Default|GetbPanning)) (Utilities|IsValid _followactor))
    (Transformation|SetActorLocation (Transformation|GetActorLocation _followactor) false false)))

(fn ConstructionScript
  (bind _returnvalue (Actor|GetActorOfClass "/Game/Core/GridCombat/BP_GridManager.BP_GridManager_C"))
  (Variables|Default|SetGridManagerRef _returnvalue)
  (CallFunction|SetCameraBounds))

(fn SetCameraBounds
  (bind _gridmanagerref (Variables|Default|GetGridManagerRef))
  (bind _gridsize (Variables|/Game/Core/GridCombat/BP_GridManager.BP_GridManager_C|GetGridSize _gridmanagerref))
  (bind _tilesize (Variables|/Game/Core/GridCombat/BP_GridManager.BP_GridManager_C|GetTileSize _gridmanagerref))
  (bind _returnvalue (/ _tilesize 2.0))
  (Variables|Default|SetMaxCameraBounds (Math|Vector|MakeVector (- (* (.x _gridsize) _tilesize) _returnvalue) (- (* (.y _gridsize) _tilesize) _returnvalue) 0.0))
  (Variables|Default|SetMinCameraBounds (Math|Vector|MakeVector _returnvalue _returnvalue 0.0)))