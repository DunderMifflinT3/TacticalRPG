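; BP_CombatInstance is a short-lived actor that runs one grid combat exchange for an initiating ability, then destroys itself.
; It notifies the owning unit and units on connected indexes, adds those units to the ability's target map, and waits while the ability animates.
; EndCombat then messages all participants.
; Counterattacks and combat simulation are stubs: both counter branches end combat, CanTargetCounter only checks range pattern, and SimulateCombatOnUnit returns zeros.
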(event Custom|EnterCombat
  (Class|BPICombatInteraction|OnUnitInitiate(Message) (Variables|/Game/Core/GridCombat/Units/Abilities/Abilities/BP_Ability.BP_Ability_C|GetOwningUnit (Variables|Default|GetInitiatingAbility)) (Variables|Default|GetInitiatingAbility))
  (for _array_element (Default|GetConnectedIndexes (Variables|Default|GetInitiatingAbility) (Variables|/Game/Core/GridCombat/BP_GridActor.BP_GridActor_C|GetGridIndex (Variables|/Game/Core/GridCombat/Units/Abilities/Abilities/BP_Ability.BP_Ability_C|GetOwningUnit (Variables|Default|GetInitiatingAbility))) (Variables|Default|GetTargetIndex))
    (Class|BPICombatInteraction|OnFoeInitiate(Message) (.unit (Default|GetIndexAttributes (Variables|/Game/Core/GridCombat/Units/Abilities/Abilities/BP_Ability.BP_Ability_C|GetGridManagerRef (Variables|Default|GetInitiatingAbility)) _array_element)) (Variables|Default|GetInitiatingAbility))
    (Default|AddtoTargetMap (Variables|Default|GetInitiatingAbility) (.unit (Default|GetIndexAttributes (Variables|/Game/Core/GridCombat/Units/Abilities/Abilities/BP_Ability.BP_Ability_C|GetGridManagerRef (Variables|Default|GetInitiatingAbility)) _array_element))))
  (Class|BPIAbilityInteraction|AnimateAbility(Message) (Variables|Default|GetInitiatingAbility) (Variables|Default|GetTargetIndex))
  (Utilities|DelayWhile (Variables|/Game/Core/GridCombat/Units/Abilities/Abilities/BP_Ability.BP_Ability_C|GetbAnimating (Variables|Default|GetInitiatingAbility))
    (:Continue
      (if (Variables|/Game/Core/GridCombat/Units/Abilities/Abilities/BP_Ability.BP_Ability_C|GetbCanBeCountered (Variables|Default|GetInitiatingAbility))
        (CallFunction|EndCombat)
        (else
          (CallFunction|EndCombat))))))

(event Custom|EndCombat
  (Class|BPICombatInteraction|OnEndCombat(Message) (Variables|/Game/Core/GridCombat/Units/Abilities/Abilities/BP_Ability.BP_Ability_C|GetOwningUnit (Variables|Default|GetInitiatingAbility)) (Variables|Default|GetInitiatingAbility))
  (bind _keys (Utilities|Map|Keys (Variables|/Game/Core/GridCombat/Units/Abilities/Abilities/BP_Ability.BP_Ability_C|GetTargetMap (Variables|Default|GetInitiatingAbility))))
  (for _array_element _keys
    (Utilities|IsValid _array_element
      (:Is%20Valid
        (Class|BPICombatInteraction|OnEndCombat(Message) _array_element (Variables|Default|GetInitiatingAbility)))))
  (Actor|DestroyActor))

(fn ConstructionScript)

(fn CanTargetCounter
  (params (Target :type BP%20Unit%20Object%20Reference))
  (return (Utilities|Enum|Equal(Enum) (Variables|/Game/Core/GridCombat/Units/Abilities/Abilities/BP_Ability.BP_Ability_C|GetRangePattern (Variables|Default|GetInitiatingAbility)) "NewEnumerator5")))

(fn SimulateCombatonUnit
  (params (Target :type BP%20Unit%20Object%20Reference) (Ability :type BP%20Ability%20Object%20Reference))
  (return (Utilities|Struct|MakeFDamage 0 0 0)))