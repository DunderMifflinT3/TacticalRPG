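; BP_GridUI is the visual feedback actor for grid combat, showing tile highlights, path, hover marker and hovered-unit data.
; Move, attack and heal ranges share one instanced mesh component, whose mesh is swapped on each highlight, with indices stored per type for removal.
; The path is a linear-point spline that can report its highest Z.
; A W_UnitData widget, created at BeginPlay, is repositioned and shown for valid hovered units.
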(event EventBeginPlay
  (bind _returnvalue (UserInterface|CreateWidget "/Game/Core/GridCombat/UI/W_UnitData.W_UnitData_C" 0 0))
  (bind _output_get (Variables|Default|SetUnitData _returnvalue))
  (UserInterface|SetWidget (Variables|Default|GetHoveredUnitData) _output_get))

(event Collision|EventActorBeginOverlap
  (params (OtherActor :type Actor%20Object%20Reference)))

(event EventTick
  (params (DeltaSeconds :type Float%20%28single-precision%29)))

(fn ConstructionScript)

(fn HighlightTiles
  (params (Locations :type Array%20of%20Transforms) (HighlightType :type EHighlightType%20Enum :default "NewEnumerator0"))
  (Components|StaticMesh|SetStaticMesh (Variables|Default|GetHighlightedTiles) (CallFunction|GetHighlightMesh HighlightType))
  (bind _returnvalue (Components|InstancedStaticMesh|AddInstances (Variables|Default|GetHighlightedTiles) Locations true))
  (switch Utilities|FlowControl|Switch|SwitchonEHighlightType HighlightType
    (:NewEnumerator0
      (Variables|Default|SetHighlightedMove _returnvalue))
    (:NewEnumerator1
      (Variables|Default|SetHighlightedAttack _returnvalue))
    (:NewEnumerator2
      (Variables|Default|SetHighlightedHeal _returnvalue))))

(fn RemoveHighlightedTiles
  (params (HighlightType :type EHighlightType%20Enum :default "NewEnumerator0"))
  (switch Utilities|FlowControl|Switch|SwitchonEHighlightType HighlightType
    (:NewEnumerator0
      (Class|HierarchicalInstancedStaticMeshComponent|RemoveInstances (Variables|Default|GetHighlightedTiles) (Variables|Default|GetHighlightedMove)))
    (:NewEnumerator1
      (Class|HierarchicalInstancedStaticMeshComponent|RemoveInstances (Variables|Default|GetHighlightedTiles) (Variables|Default|GetHighlightedAttack)))
    (:NewEnumerator2
      (Class|HierarchicalInstancedStaticMeshComponent|RemoveInstances (Variables|Default|GetHighlightedTiles) (Variables|Default|GetHighlightedHeal)))))

(fn GetHighlightMesh
  (params (HighlightType :type EHighlightType%20Enum :default "NewEnumerator0"))
  (return (Utilities|Select :Index HighlightType :NewEnumerator0 (Variables|Default|GetMoveRange) :NewEnumerator1 (Variables|Default|GetAttackRange) :NewEnumerator2 (Variables|Default|GetHealRange))))

(fn AddPathSplinePoint
  (params (Locations :type Array%20of%20Vectors))
  (bind _pathspline (Variables|Default|GetPathSpline))
  (for (_array_element _array_index) Locations
    (Spline|AddSplinePointatIndex _pathspline _array_element _array_index "World" true)
    (Spline|SetSplinePointType _pathspline _array_index "Linear" true)))

(fn ClearPathSpline
  (Spline|ClearSplinePoints (Variables|Default|GetPathSpline) true))

(fn SetHoverMarkerTransform
  (params (Location :type Vector))
  (Transformation|SetWorldTransform (Variables|Default|GetHoverMarker) (Math|Transform|MakeTransform (Math|Vector|MakeVector (.x Location) (.y Location) (+ (.z Location) 0.021)) "0, 0, 0" "1,1,1") false false))

(fn SetHoverMarkerVisibility
  (params (Visible :type Boolean))
  (Rendering|SetVisibility (Variables|Default|GetHoverMarker) Visible false))

(fn GetMaxZCoordonPath
  (for _index (range 0 (- (Spline|GetNumberOfSplinePoints (Variables|Default|GetPathSpline)) 1))
    (if (> (.z (Spline|GetLocationatSplinePoint (Variables|Default|GetPathSpline) _index "World")) (LocalVariables|GetLMaxZ))
      (LocalVariables|SetLMaxZ (.z (Spline|GetLocationatSplinePoint (Variables|Default|GetPathSpline) _index "World")))))
  (return (LocalVariables|GetLMaxZ)))

(fn UpdateHoveredUnitData
  (params (Unit :type BP%20Unit%20Object%20Reference) (Location :type Vector))
  (Utilities|IsValid Unit
    (:Is%20Valid
      (Variables|/Game/Core/GridCombat/UI/W_UnitData.W_UnitData_C|SetOwningUnit (Variables|Default|GetUnitData) Unit)
      (Transformation|SetRelativeLocation (Variables|Default|GetHoveredUnitData) Location false false)
      (Rendering|SetVisibility (Variables|Default|GetHoveredUnitData) true false))
    (:Is%20Not%20Valid
      (Rendering|SetVisibility (Variables|Default|GetHoveredUnitData) false false)
      (Variables|/Game/Core/GridCombat/UI/W_UnitData.W_UnitData_C|SetOwningUnit (Variables|Default|GetUnitData) 0))))