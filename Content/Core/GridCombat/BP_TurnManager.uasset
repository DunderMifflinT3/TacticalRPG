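; Turn manager for grid combat that cycles faction phases and tracks which units still have to act.
; BeginCombat gathers factions from units on the field, then each phase shows the HUD banner, refreshes that faction's units and advances when none remain.
; AI units activate one after another, while player units wait for a camera pan with input locked.
; Helpers derive the turn number from phase count and handle faction changes and deaths.
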(event Custom|EndActiveFactionTurn
  (Default|ToggleInput (Variables|Default|GetPlayerController) false)
  (if (> (Utilities|Array|Length (Variables|Default|GetUnitsToAct)) 0)
    ;[1 1 1] Ends the turn of each unit that still needs to act
    (for _array_element (Variables|Default|GetUnitsToAct)
      (Class|BPIInitiative|EndTurn(Message) _array_element)
      (Utilities|Array|RemoveItem (Variables|Default|GetUnitsToAct) _array_element)))
  (if (== (Utilities|Array|LastIndex (Variables|Default|GetFactions)) (Utilities|Array|FindItem (Variables|Default|GetFactions) (Variables|Default|GetActiveFaction)))
    ;[1 1 1] Sets active faction to first element if last active faction was the last element
    (Variables|Default|SetActiveFaction (Utilities|Array|Get(acopy) (Variables|Default|GetFactions)))
    (else
      ;[1 1 1] Sets active faction to the next one in the array
      (Variables|Default|SetActiveFaction (Utilities|Array|Get(acopy) (Variables|Default|GetFactions) (+ (Utilities|Array|FindItem (Variables|Default|GetFactions) (Variables|Default|GetActiveFaction)) 1)))))
  (CallFunction|BeginActiveFactionTurn))

(event Custom|BeginActiveFactionTurn
  (bind _gridmanagerref (Variables|Default|GetGridManagerRef))
  (bind _activefaction (Variables|Default|GetActiveFaction))
  (bind _unitsoffaction (CallFunction|GetAllUnitsOfFaction _activefaction))
  (bind _combathudref (Variables|/Game/Core/GridCombat/BP_GridManager.BP_GridManager_C|GetCombatHUDRef _gridmanagerref))
  (Math|Integer|IncrementInt (Variables|Default|GetTotalPhases)
    (:%20%20
      (Default|PhaseChange _combathudref (Variables|Default|GetActiveFaction) (CallFunction|GetTurnNumber))
      (Utilities|DelayWhile (Widget|IsVisible (Variables|/Game/Core/GridCombat/UI/W_CombatHUD.W_CombatHUD_C|GetW_PhaseChange _combathudref))
        (:Continue
          ;[1 1 1] Checks if there are any units left in the new active faction
          (if (> (Utilities|Array|Length _unitsoffaction) 0)
            (bind _output_get (Variables|Default|SetUnitsToAct _unitsoffaction))
            (for _array_element _output_get
              (Utilities|IsValid _array_element
                (:Is%20Valid
                  (Class|BPIInitiative|BeginTurn(Message) _array_element))))
            (CallFunction|CheckforUnitstoAct)
            (else
              (CallFunction|EndActiveFactionTurn))))))))

(event Custom|BeginCombat
  (Variables|Default|SetPlayerFaction (Variables|Default|GetActiveFaction))
  (bind _asplayer_controller_grid (Utilities|Casting|CastToPlayerController_Grid (Game|GetPlayerController 0)))
  (bind _output_get (Variables|Default|SetPlayerController _asplayer_controller_grid))
  (Default|ToggleInput _output_get false)
  (for _array_element (Variables|Default|GetUnitsOnField)
    (if (not (Utilities|Array|ContainsItem (Variables|Default|GetFactions) (Default|GetUnitFaction _array_element)))
      (Utilities|Array|Add (Variables|Default|GetFactions) (Default|GetUnitFaction _array_element))))
  (CallFunction|BeginActiveFactionTurn))

(event Custom|ActivateUnit
  (params (Unit :type BP%20Unit%20Object%20Reference))
  (bind _gridmanagerref (Variables|Default|GetGridManagerRef))
  (bind _gridcamera (Variables|/Game/Core/GridCombat/BP_GridManager.BP_GridManager_C|GetGridCamera _gridmanagerref))
  (if (Default|CanAct Unit)
    (if (Utilities|Enum|Equal(Enum) (Default|GetUnitFaction Unit) (Variables|Default|GetActiveFaction))
      (bind _output_get (Variables|Default|SetActiveUnit Unit))
      (if (not (Default|IsAIControlled _output_get))
        (Default|ToggleInput (Variables|Default|GetPlayerController) false)
        ;[1 1 1] Wait for camera to pan to unit
        (Default|PantoActor _gridcamera (Variables|Default|GetActiveUnit))
        (Utilities|DelayWhile (Variables|/Game/Core/GridCombat/BP_GridCamera.BP_GridCamera_C|GetbPanning _gridcamera)
          (:Continue
            (Default|ToggleInput (Variables|Default|GetPlayerController) true)
            (Class|BPIInitiative|Activate(Message) (Variables|Default|GetActiveUnit))))
        (else
          (Class|BPIInitiative|Activate(Message) (Variables|Default|GetActiveUnit)))))))

(event Custom|EndUnitTurn
  (params (Unit :type BP%20Unit%20Object%20Reference))
  (Class|BPIInitiative|EndTurn(Message) Unit)
  (Utilities|Array|RemoveItem (Variables|Default|GetUnitsToAct) Unit)
  (Variables|Default|SetActiveUnit 0)
  (CallFunction|CheckforUnitstoAct))

(event Custom|DeactivateUnit
  (params (Unit :type BP%20Unit%20Object%20Reference))
  (Class|BPIInitiative|Deactivate(Message) Unit)
  (Variables|Default|SetActiveUnit 0))

(event Custom|CheckForUnitsToAct
  (if (<= (Utilities|Array|Length (Variables|Default|GetUnitsToAct)) 0)
    (CallFunction|EndActiveFactionTurn)
    (elif (Utilities|Enum|NotEqual(Enum) (Variables|Default|GetActiveFaction) (Variables|Default|GetPlayerFaction))
      (Default|ToggleInput (Variables|Default|GetPlayerController) false)
      ;[1 1 1] Activates next AI unit
      (bind _array_element (Utilities|Array|ForEachLoopwithBreak (Variables|Default|GetUnitsToAct) :!label _label)
        (:LoopBody
          (if (Default|CanAct _array_element)
            (CallFunction|ActivateUnit _array_element)
            (goto _label Break))))
      (else
        (Default|ToggleInput (Variables|Default|GetPlayerController) true)))))

(fn ConstructionScript)

(fn GetAllUnitsOfFaction
  (params (Faction :type EFaction%20Enum :default "NewEnumerator0"))
  (for _array_element (Variables|Default|GetUnitsOnField)
    (if (Utilities|Enum|Equal(Enum) (Default|GetUnitFaction _array_element) Faction)
      (Utilities|Array|Add (LocalVariables|GetLUnitsOfFaction) _array_element)))
  (return (LocalVariables|GetLUnitsOfFaction)))

(fn GetTurnNumber
  (return (+ (/ (- (Variables|Default|GetTotalPhases) 1) (Utilities|Array|Length (Variables|Default|GetFactions))) 1)))

(fn ChangeUnitFaction
  (params (Unit :type BP%20Unit%20Object%20Reference) (NewFaction :type EFaction%20Enum :default "NewEnumerator0"))
  (Default|UpdateFaction Unit NewFaction)
  (if (Utilities|Enum|Equal(Enum) (Variables|Default|GetActiveFaction) NewFaction)
    (Utilities|Array|Add (Variables|Default|GetUnitsToAct) Unit)))

(fn KillUnit
  (params (Unit :type BP%20Unit%20Object%20Reference))
  (Utilities|Array|RemoveItem (Variables|Default|GetUnitsOnField) Unit)
  (Utilities|Array|RemoveItem (Variables|Default|GetUnitsToAct) Unit))