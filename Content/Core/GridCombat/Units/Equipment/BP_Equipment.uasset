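; BP_Equipment is an equipment item for grid combat units that supplies stat, combat stat and growth modifiers.
; Equip and Unequip only set or clear the OwningUnit reference, without applying any modifiers themselves.
; Three getters look up the modifier for a given stat in their respective maps.
; CanBeEquipped accepts every unit, with no restrictions in this Blueprint.
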(event EventEquip
  (params (Unit :type BP%20Unit%20Object%20Reference))
  (Variables|Default|SetOwningUnit Unit))

(event EventUnequip
  (Variables|Default|SetOwningUnit 0))

(fn ConstructionScript)

(fn GetStatModifier
  (params (Stat :type EStats%20Enum :default "NewEnumerator9"))
  (return (.Value (Utilities|Map|Find (Variables|Default|GetStatModifiers) Stat))))

(fn GetCombatStatModifier
  (params (Stat :type ECombatStats%20Enum :default "NewEnumerator7"))
  (return (.Value (Utilities|Map|Find (Variables|Default|GetCombatStatModifiers) Stat))))

(fn GetGrowthModifier
  (params (Stat :type EStats%20Enum :default "NewEnumerator9"))
  (return (.Value (Utilities|Map|Find (Variables|Default|GetGrowthModifiers) Stat))))

(fn CanbeEquipped
  (params (Unit :type BP%20Unit%20Object%20Reference))
  (return true))