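; BP_Mount is a mount equipment item for grid-combat units, carrying movement, stat, terrain, ability and passive data.
; Its construction script loads all of these fields from the DT_MountData row matching its InternalName.
; CanBeEquipped passes if any of the unit's class types is in the mount's allowed ClassTypes.
; GetTerrainCost looks up the terrain cost map and returns a prohibitive default for unlisted terrain.
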(fn ConstructionScript
  (bind _returnvalue (Utilities|GetDataTableRow "/Game/Core/GridCombat/Units/Equipment/Mounts/DT_MountData.DT_MountData" (Variables|Default|GetInternalName))
    (:then
      (Variables|Default|SetName (.name _returnvalue))
      (Variables|Default|SetDescription (.description _returnvalue))
      (Variables|Default|SetClassTypes (.classtypes _returnvalue))
      (Variables|Default|SetMove (.move _returnvalue))
      (Variables|Default|SetJump (.jump _returnvalue))
      (Variables|Default|SetStatModifiers (.statmodifiers _returnvalue))
      (Variables|Default|SetCombatStatModifiers (.combatstatmodifiers _returnvalue))
      (Variables|Default|SetGrowthModifiers (.growthmodifiers _returnvalue))
      (Variables|Default|SetTerrainCosts (.terraincost _returnvalue))
      (Variables|Default|SetDamageModifiers (.damagemodifiers _returnvalue))
      (Variables|Default|SetbFlying (.flying _returnvalue))
      (Variables|Default|SetAbilities (.abilities _returnvalue))
      (Variables|Default|SetPassives (.passives _returnvalue))
      (Variables|Default|SetCost (.cost _returnvalue)))))

(fn CanbeEquipped
  (params (Unit :type BP%20Unit%20Object%20Reference))
  (for _array_element (Default|GetClassType (Variables|/Game/Core/GridCombat/Units/BP_Unit.BP_Unit_C|GetClassComponent Unit))
    (if (Utilities|Array|ContainsItem (Variables|Default|GetClassTypes) _array_element)
      (return true)))
  (return false))

(fn GetTerrainCost
  (params (Terrain :type ETerrain%20Enum :default "NewEnumerator0"))
  (bind _terraincosts (Variables|Default|GetTerrainCosts))
  (bind (_value _returnvalue) (Utilities|Map|Find _terraincosts Terrain))
  (if _returnvalue
    (return _value)
    (else
      (return 999))))