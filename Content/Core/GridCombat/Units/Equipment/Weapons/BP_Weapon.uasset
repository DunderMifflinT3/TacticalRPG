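; BP_Weapon represents a unit's weapon in grid combat, holding its combat stats, range, usage rules, abilities, passives and cost.
; The construction script looks up InternalName in DT_WeaponData and copies the row's fields into the weapon's variables, so each weapon is data-driven.
; CanBeEquipped checks whether the weapon's type is among the usable weapons reported by the unit's ClassComponent.
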(fn ConstructionScript
  (bind _returnvalue (Utilities|GetDataTableRow "/Game/Core/GridCombat/Units/Equipment/Weapons/DT_WeaponData.DT_WeaponData" (Variables|Default|GetInternalName))
    (:then
      (Variables|Default|SetName (.name _returnvalue))
      (Variables|Default|SetDescription (.description _returnvalue))
      (Variables|Default|SetWeaponType (.weapontype _returnvalue))
      (Variables|Default|SetDamageType (.damagetype _returnvalue))
      (Variables|Default|SetAttackStat (.attackstat _returnvalue))
      (Variables|Default|SetDefendStat (.defendstat _returnvalue))
      (Variables|Default|SetCombatStatModifiers (.combatstats _returnvalue))
      (Variables|Default|SetCriticalModifier (.criticalmodifier _returnvalue))
      (Variables|Default|SetMinRange (.minrange _returnvalue))
      (Variables|Default|SetMaxRange (.maxrange _returnvalue))
      (Variables|Default|SetVerticalRange (.verticalrange _returnvalue))
      (Variables|Default|SetWeight (.weight _returnvalue))
      (Variables|Default|SetStatModifiers (.statmodifiers _returnvalue))
      (Variables|Default|SetGrowthModifiers (.growthmodifiers _returnvalue))
      (Variables|Default|SetbDiagonal (.diagonalrange _returnvalue))
      (Variables|Default|SetbUseWithShield (.usewithshield _returnvalue))
      (Variables|Default|SetbUseWithMount (.usewithmount _returnvalue))
      (Variables|Default|SetbUseMagic (.canusemagic _returnvalue))
      (Variables|Default|SetbEffectiveOnFlying (.effectiveonflying _returnvalue))
      (Variables|Default|SetbEffectiveOnMounted (.effectiveonmounted _returnvalue))
      (Variables|Default|SetbCanBeCountered (.canbecountered _returnvalue))
      (Variables|Default|SetAttackAbility (.attackability _returnvalue))
      (Variables|Default|SetCounterAbility (.counterability _returnvalue))
      (Variables|Default|SetAbilities (.abilities _returnvalue))
      (Variables|Default|SetPassives (.passives _returnvalue))
      (Variables|Default|SetCost (.cost _returnvalue)))))

(fn CanbeEquipped
  (params (Unit :type BP%20Unit%20Object%20Reference))
  (return (Utilities|Array|ContainsItem (Default|GetUsableWeapons (Variables|/Game/Core/GridCombat/Units/BP_Unit.BP_Unit_C|GetClassComponent Unit)) (Variables|Default|GetWeaponType))))