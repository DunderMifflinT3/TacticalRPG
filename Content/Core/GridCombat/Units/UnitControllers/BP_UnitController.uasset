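; Base controller for a unit in grid combat, handling its activation, move range and action menu.
; Activation caches reachable grid indexes from the grid manager and spawns each active ability as an actor, sorted into valid or invalid lists by CanActivate.
; Ending the action destroys those ability actors.
; Show and hide functions toggle the combat HUD's unit action widget and the grid player controller's input.
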(event Custom|ActivateUnit
  (bind _owningunit (Variables|Default|GetOwningUnit))
  (Utilities|Array|Clear (Variables|Default|GetValidAbilities))
  (Utilities|Array|Clear (Variables|Default|GetInvalidAbilities))
  (Variables|Default|SetIndexesInRange (CallFunction|GetIndexesinMoveRange (Variables|/Game/Core/GridCombat/BP_GridActor.BP_GridActor_C|GetGridIndex (Variables|Default|GetOwningUnit))))
  (for _array_element (Default|GetActiveAbilities _owningunit)
    (bind _returnvalue (Game|SpawnActorfromClass _array_element (Math|Transform|MakeTransform "0, 0, 0" "0, 0, 0" "1.000000,1,1") "AlwaysSpawn" 0 _owningunit 0))
    (if (Default|CanActivate _returnvalue)
      (Utilities|Array|Add (Variables|Default|GetValidAbilities) _returnvalue)
      (else
        (Utilities|Array|Add (Variables|Default|GetInvalidAbilities) _returnvalue)))))

(event Custom|EndUnitAction
  (for _array_element (Variables|Default|GetValidAbilities)
    (Utilities|IsValid _array_element
      (:Is%20Valid
        (Actor|DestroyActor _array_element))))
  (for _array_element_2 (Variables|Default|GetInvalidAbilities)
    (Utilities|IsValid _array_element_2
      (:Is%20Valid
        (Actor|DestroyActor _array_element_2)))))

(fn ConstructionScript
  (Variables|Default|SetGridManagerRef (Variables|/Game/Core/GridCombat/BP_GridActor.BP_GridActor_C|GetGridManagerRef (Variables|Default|GetOwningUnit))))

(fn GetIndexesinMoveRange
  (params (StartIndex :type F%20Grid%20Index%20Structure))
  (return (Default|FindReachableIndexes (Variables|Default|GetGridManagerRef) (Variables|Default|GetOwningUnit) StartIndex)))

(fn ShowUnitActions
  (bind _gridmanagerref (Variables|Default|GetGridManagerRef))
  (bind _combathudref (Variables|/Game/Core/GridCombat/BP_GridManager.BP_GridManager_C|GetCombatHUDRef _gridmanagerref))
  (bind _w_unitactions (Variables|/Game/Core/GridCombat/UI/W_CombatHUD.W_CombatHUD_C|GetW_UnitActions _combathudref))
  (bind _asplayer_controller_grid (Utilities|Casting|CastToPlayerController_Grid (Game|GetPlayerController 0)))
  (Default|ToggleInput _asplayer_controller_grid false)
  (Default|SetSprite (Variables|Default|GetOwningUnit) "NewEnumerator3" 9e+01)
  (Variables|/Game/Core/GridCombat/UI/W_UnitActions.W_UnitActions_C|SetActiveUnit _w_unitactions (Variables|Default|GetOwningUnit))
  (Widget|SetVisibility _w_unitactions "Visible"))

(fn HideUnitActions
  (Widget|SetVisibility (Variables|/Game/Core/GridCombat/UI/W_CombatHUD.W_CombatHUD_C|GetW_UnitActions (Variables|/Game/Core/GridCombat/BP_GridManager.BP_GridManager_C|GetCombatHUDRef (Variables|Default|GetGridManagerRef))) "Collapsed")
  (Variables|/Game/Core/GridCombat/UI/W_UnitActions.W_UnitActions_C|SetActiveUnit (Variables|/Game/Core/GridCombat/UI/W_CombatHUD.W_CombatHUD_C|GetW_UnitActions (Variables|/Game/Core/GridCombat/BP_GridManager.BP_GridManager_C|GetCombatHUDRef (Variables|Default|GetGridManagerRef))) 0)
  (bind _asplayer_controller_grid (Utilities|Casting|CastToPlayerController_Grid (Game|GetPlayerController 0)))
  (Default|ToggleInput _asplayer_controller_grid true))