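; AI controller for a grid-combat unit that picks and performs the unit's action on its turn.
; On activation it finds units in ability range, then scores every ability, reachable tile and target combination.
; Scores sum ability power on valid targets, penalize other hits double, and break ties by shortest path.
; It pans the camera, moves, executes the best ability and ends the turn, or just ends it if nothing scores positively.
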(event EventEndUnitAction
  (Variables|Default|SetBestScore 0)
  (Variables|Default|SetBestTarget (Utilities|Struct|MakeFGridIndex -1 -1))
  (Variables|Default|SetBestMoveTarget (Utilities|Struct|MakeFGridIndex -1 -1))
  (Variables|Default|SetShortestPath 0)
  (Variables|Default|SetSelectedAbility 0)
  (Utilities|Set|Clear (Variables|Default|GetUnitsInRange))
  (|CallParentFunction)
  (Default|EndUnitTurn (Variables|/Game/Core/GridCombat/BP_GridManager.BP_GridManager_C|GetTurnManagerRef (Variables|Default|GetGridManagerRef)) (Variables|Default|GetOwningUnit)))

(event EventActivateUnit
  (bind _gridmanagerref (Variables|Default|GetGridManagerRef))
  (bind _owningunit (Variables|Default|GetOwningUnit))
  (bind _owningunit_2 (Variables|Default|GetOwningUnit))
  (bind _owningunit_3 (Variables|Default|GetOwningUnit))
  (bind _gridcamera (Variables|/Game/Core/GridCombat/BP_GridManager.BP_GridManager_C|GetGridCamera _gridmanagerref))
  (|CallParentFunction)
  ;[1 1 1] Adds basic attack to the list of potential abilities
  (bind _returnvalue (Game|SpawnActorfromClass (Default|GetAttackAbility _owningunit_2) (Math|Transform|MakeTransform "0, 0, 0" "0, 0, 0" "1,1,1") "AlwaysSpawn" 0 _owningunit_2 0))
  (if (Default|CanActivate _returnvalue)
    (Utilities|Array|Add (Variables|Default|GetValidAbilities) _returnvalue)
    (else
      (Utilities|Array|Add (Variables|Default|GetInvalidAbilities) _returnvalue)))
  (for _array_element (Variables|Default|GetIndexesInRange)
    ;[1 1 1] Finds all units in range of any abilities
    (for _array_element_2 (Variables|Default|GetValidAbilities)
      (bind (_unitsinrange _unitsfound) (CallFunction|FindUnitsinRange _array_element _array_element_2))
      (if _unitsfound
        (Utilities|Set|AddItems (Variables|Default|GetUnitsInRange) _unitsinrange))))
  ;[1 1 1] Checks if any units are in range
  (if (> (Utilities|Set|Length (Variables|Default|GetUnitsInRange)) 0)
    (bind _result (Utilities|Set|ToArray (Variables|Default|GetUnitsInRange)))
    (for _array_element_3 _result
      (for _array_element_4 (Variables|Default|GetValidAbilities)
        ;[1 1 1] Checks if the target is of the relevant faction
        (if (CallFunction|IsUnitValidTarget _array_element_3 _array_element_4)
          ;[1 1 1] Gets indexes in ability's range from the target, resulting in potential move targets for the ability to be used from
          (for _array_element_5 (Default|GetIndexesinRange _array_element_4 (Variables|/Game/Core/GridCombat/BP_GridActor.BP_GridActor_C|GetGridIndex _array_element_3))
            ;[1 1 1] Checks if index can be moved to
            (if (Utilities|Array|ContainsItem (Variables|Default|GetIndexesInRange) _array_element_5)
              ;[1 1 1] Evaluates usefulness of this ability on this target
              (bind _score (CallFunction|EvaluateTarget _array_element_4 _array_element_5 (Variables|/Game/Core/GridCombat/BP_GridActor.BP_GridActor_C|GetGridIndex _array_element_3)))
              (if (> _score (Variables|Default|GetBestScore))
                ;[1 1 1] Sets the length of the path to the target, in case other indexes have the same score
                (Variables|Default|SetShortestPath (.PathCost (Default|FindPathtoIndex (Variables|Default|GetGridManagerRef) _owningunit (Variables|/Game/Core/GridCombat/BP_GridActor.BP_GridActor_C|GetGridIndex _owningunit) _array_element_5)))
                ;[0 1 0] Updates best move
                (Variables|Default|SetSelectedAbility _array_element_4 :!label _label)
                (Variables|Default|SetBestScore _score)
                (Variables|Default|SetBestMoveTarget _array_element_5)
                (Variables|Default|SetBestTarget (Variables|/Game/Core/GridCombat/BP_GridActor.BP_GridActor_C|GetGridIndex _array_element_3))
                (else
                  ;[1 1 1] Prioritizes shortest path to target if the score is the same
                  (if (== _score (Variables|Default|GetBestScore))
                    (if (< (.PathCost (Default|FindPathtoIndex (Variables|Default|GetGridManagerRef) _owningunit_3 (Variables|/Game/Core/GridCombat/BP_GridActor.BP_GridActor_C|GetGridIndex _owningunit_3) _array_element_5)) (Variables|Default|GetShortestPath))
                      (Variables|Default|SetShortestPath (.PathCost (Default|FindPathtoIndex (Variables|Default|GetGridManagerRef) _owningunit_3 (Variables|/Game/Core/GridCombat/BP_GridActor.BP_GridActor_C|GetGridIndex _owningunit_3) _array_element_5)))
                      (goto _label))))))))))
    ;[1 1 1] Checks if any moves are worth it
    (if (and (> (Variables|Default|GetBestScore) 0) (Utilities|IsValid (Variables|Default|GetSelectedAbility)))
      ;[1 1 1] Pans to unit if they will move
      (Default|PantoActor _gridcamera (Variables|Default|GetOwningUnit))
      (Utilities|DelayWhile (Variables|/Game/Core/GridCombat/BP_GridCamera.BP_GridCamera_C|GetbPanning _gridcamera)
        (:Continue
          ;[1 1 1] Moves unit to the target index
          (bind _returnvalue_2 (Game|SpawnActorfromClass "/Game/Core/GridCombat/Units/Abilities/Abilities/BP_Ability_Move.BP_Ability_Move_C" (Math|Transform|MakeTransform "0, 0, 0" "0, 0, 0" "1,1,1") "AlwaysSpawn" 0 (Variables|Default|GetOwningUnit) 0))
          (Class|BPIAbilityInteraction|ExecuteAbility(Message) _returnvalue_2 (Variables|Default|GetBestMoveTarget))
          (Utilities|DelayWhile (Utilities|IsValid _returnvalue_2)
            (:Continue
              ;[1 1 1] Performs unit's chosen ability
              (Class|BPIAbilityInteraction|ActivateAbility(Message) (Variables|Default|GetSelectedAbility))
              (Class|BPIAbilityInteraction|ExecuteAbility(Message) (Variables|Default|GetSelectedAbility) (Variables|Default|GetBestTarget))
              (Utilities|DelayWhile (Utilities|IsValid (Variables|Default|GetSelectedAbility))
                (:Continue
                  (CallFunction|EndUnitAction)))))))
      (else
        ;[1 0 0] No valid moves
        (CallFunction|EndUnitAction :!label _label_2)))
    (else
      (goto _label_2))))

(fn ConstructionScript
  (|CallParentFunction))

(fn EvaluateTarget
  (params (Ability :type BP%20Ability%20Object%20Reference) (MoveIndex :type F%20Grid%20Index%20Structure) (TargetIndex :type F%20Grid%20Index%20Structure))
  (for _array_element (Default|GetConnectedIndexes Ability MoveIndex TargetIndex)
    (if (CallFunction|IsUnitValidTarget (.unit (Default|GetIndexAttributes (Variables|Default|GetGridManagerRef) _array_element)) Ability)
      (LocalVariables|SetLScore (+ (Default|CalculatePower Ability (.unit (Default|GetIndexAttributes (Variables|Default|GetGridManagerRef) _array_element))) (LocalVariables|GetLScore)))
      (else
        (LocalVariables|SetLScore (- (LocalVariables|GetLScore) (* (Default|CalculatePower Ability (.unit (Default|GetIndexAttributes (Variables|Default|GetGridManagerRef) _array_element))) 2))))))
  (return (LocalVariables|GetLScore)))

(fn FindUnitsinRange
  (params (Index :type F%20Grid%20Index%20Structure) (Ability :type BP%20Ability%20Object%20Reference))
  (Utilities|IsValid Ability
    (:Is%20Valid
      (for _array_element (Default|GetIndexesinRange Ability Index)
        (Utilities|IsValid (.unit (Default|GetIndexAttributes (Variables|Default|GetGridManagerRef) _array_element))
          (:Is%20Valid
            (Utilities|Array|Add (LocalVariables|GetLUnitsInRange) (.unit (Default|GetIndexAttributes (Variables|Default|GetGridManagerRef) _array_element))))))
      (return (LocalVariables|GetLUnitsInRange) (> (Utilities|Array|Length (LocalVariables|GetLUnitsInRange)) 0)))))

(fn IsUnitValidTarget
  (params (TargetUnit :type BP%20Unit%20Object%20Reference) (Ability :type BP%20Ability%20Object%20Reference))
  (Utilities|IsValid TargetUnit
    (:Is%20Valid
      (Utilities|IsValid Ability
        (:Is%20Valid
          (if (Variables|/Game/Core/GridCombat/Units/Abilities/Abilities/BP_Ability.BP_Ability_C|GetbTargetAllies Ability)
            (if (Variables|/Game/Core/GridCombat/Units/Abilities/Abilities/BP_Ability.BP_Ability_C|GetbTargetSelf Ability)
              (return (== (Default|GetUnitFaction (Variables|Default|GetOwningUnit)) (Default|GetUnitFaction TargetUnit)))
              (else
                (return (and (== (Default|GetUnitFaction (Variables|Default|GetOwningUnit)) (Default|GetUnitFaction TargetUnit)) (!= TargetUnit (Variables|Default|GetOwningUnit))))))
            (else
              (return (Utilities|Enum|NotEqual(Enum) (Default|GetUnitFaction (Variables|Default|GetOwningUnit)) (Default|GetUnitFaction TargetUnit))))))
        (:Is%20Not%20Valid
          _)))
    (:Is%20Not%20Valid
      _))
  (return false))