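; Unit controller for player units in grid combat, handling activation, the action menu and backing out of moves.
; On activation it snapshots grid index and status conditions, then shows the unit's actions.
; Ending an action deactivates an untouched unit, ends the turn after an action with locked movement, or otherwise reopens the menu, undoing any movement.
; Undo restores the snapshot, teleports the unit, pans the camera and clears used movement.
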(event EventActivateUnit
  (|CallParentFunction)
  (CallFunction|SaveUnitState)
  (CallFunction|ShowUnitActions))

(event EventEndUnitAction
  (bind _owningunit (Variables|Default|GetOwningUnit))
  (if (and (not (Variables|/Game/Core/GridCombat/Units/BP_Unit.BP_Unit_C|GetbUsedAction _owningunit)) (== (Variables|/Game/Core/GridCombat/Units/BP_Unit.BP_Unit_C|GetMovementUsed _owningunit) 0))
    (|CallParentFunction)
    (Default|DeactivateUnit (Variables|/Game/Core/GridCombat/BP_GridManager.BP_GridManager_C|GetTurnManagerRef (Variables|Default|GetGridManagerRef)) (Variables|Default|GetOwningUnit))
    (CallFunction|HideUnitActions)
    (else
      ;[1 1 1] Movement can only be canceled if the unit has not taken an action
      (if (not (Variables|/Game/Core/GridCombat/Units/BP_Unit.BP_Unit_C|GetbUsedAction (Variables|Default|GetOwningUnit)))
        ;[1 1 1] Resets the unit's variables to how they were when the turn started
        (CallFunction|ResetUnitState)
        (CallFunction|ShowUnitActions)
        (elif (== (Variables|/Game/Core/GridCombat/Units/BP_Unit.BP_Unit_C|GetMovementUsed (Variables|Default|GetOwningUnit)) 0)
          (CallFunction|ShowUnitActions)
          (else
            ;[1 1 1] Checks if unit should be able to cancel their movement
            (if (Variables|/Game/Core/GridCombat/Units/BP_Unit.BP_Unit_C|GetbMovementLocked (Variables|Default|GetOwningUnit))
              (|CallParentFunction)
              (Default|EndUnitTurn (Variables|/Game/Core/GridCombat/BP_GridManager.BP_GridManager_C|GetTurnManagerRef (Variables|Default|GetGridManagerRef)) (Variables|Default|GetOwningUnit))
              (else
                ;[1 1 1] Allows for movement to cancel after a unit does an action without moving
                (if (and (Variables|/Game/Core/GridCombat/Units/BP_Unit.BP_Unit_C|GetbUsedAction (Variables|Default|GetOwningUnit)) (> (Variables|/Game/Core/GridCombat/Units/BP_Unit.BP_Unit_C|GetMovementUsed (Variables|Default|GetOwningUnit)) 0))
                  ;[1 1 1] Resets unit's variables to how they were after they performed an action
                  (CallFunction|ResetUnitState)
                  (CallFunction|ShowUnitActions))))))))))

(fn ConstructionScript
  (|CallParentFunction))

(fn SaveUnitState
  (Variables|Default|SetStartingIndex (Variables|/Game/Core/GridCombat/BP_GridActor.BP_GridActor_C|GetGridIndex (Variables|Default|GetOwningUnit)))
  (Variables|Default|SetStartingStatusConditions (Variables|/Game/Core/GridCombat/Units/UnitComponents/BP_StatusComponent.BP_StatusComponent_C|GetStatusConditions (Variables|/Game/Core/GridCombat/Units/BP_Unit.BP_Unit_C|GetStatusComponent (Variables|Default|GetOwningUnit)))))

(fn ResetUnitState
  (Default|RemoveUnitfromIndex (Variables|Default|GetGridManagerRef) (Variables|/Game/Core/GridCombat/BP_GridActor.BP_GridActor_C|GetGridIndex (Variables|Default|GetOwningUnit)))
  (bind _output_get (Variables|/Game/Core/GridCombat/BP_GridActor.BP_GridActor_C|SetGridIndex (Variables|Default|GetOwningUnit) (Variables|Default|GetStartingIndex)))
  (Default|AddUnittoIndex (Variables|Default|GetGridManagerRef) _output_get (Variables|Default|GetOwningUnit))
  (Transformation|SetActorLocation (Variables|Default|GetOwningUnit) (.location (Default|GetIndexAttributes (Variables|Default|GetGridManagerRef) _output_get)) false false)
  (Default|PantoActor (Variables|/Game/Core/GridCombat/BP_GridManager.BP_GridManager_C|GetGridCamera (Variables|Default|GetGridManagerRef)) (Variables|Default|GetOwningUnit))
  (Variables|/Game/Core/GridCombat/Units/UnitComponents/BP_StatusComponent.BP_StatusComponent_C|SetStatusConditions (Variables|/Game/Core/GridCombat/Units/BP_Unit.BP_Unit_C|GetStatusComponent (Variables|Default|GetOwningUnit)) (Variables|Default|GetStartingStatusConditions))
  (Variables|/Game/Core/GridCombat/Units/BP_Unit.BP_Unit_C|SetMovementUsed (Variables|Default|GetOwningUnit) 0))