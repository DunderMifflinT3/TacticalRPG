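; Attack ability for grid combat units, targeting an occupied tile within the owner's weapon attack range.
; Execution spends stamina, marks the action used and spawns a combat instance that runs the fight.
; Animation lunges the unit sprite toward the target on a timeline, whose event triggers the ability effect.
; Afterward it waits on the combat instance, then ends execution, first updating and saving state for player units.
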(event EventAnimateAbility
  (params (Target :type F%20Grid%20Index%20Structure))
  (bind _owningunit (Variables|Default|GetOwningUnit))
  (bind _gridmanagerref (Variables|Default|GetGridManagerRef))
  (bind _gridmanagerref_2 (Variables|Default|GetGridManagerRef))
  (bind _owningunit_2 (Variables|Default|GetOwningUnit))
  (bind _owningunit_3 (Variables|Default|GetOwningUnit))
  (bind _attributes (Default|GetIndexAttributes _gridmanagerref Target))
  (bind _unitcontroller (Variables|/Game/Core/GridCombat/Units/BP_Unit.BP_Unit_C|GetUnitController _owningunit))
  (bind _gridindex (Variables|/Game/Core/GridCombat/BP_GridActor.BP_GridActor_C|GetGridIndex _owningunit_3))
  (bind _location (Utilities|Struct|BreakFGridTile _attributes))
  (bind _attributes_2 (Default|GetIndexAttributes _gridmanagerref_2 _gridindex))
  (bind _location_2 (Utilities|Struct|BreakFGridTile _attributes_2))
  (bind (_x _y) (Math|Vector|BreakVector _location_2))
  (|CallParentFunction Target)
  (Variables|Default|SetTargetPoint (+ (* (Math|Vector|GetForwardVector (Math|Rotator|FindLookatRotation _location_2 _location)) 5e+01) _location_2))
  (bind _progression (Timeline|TL_Attack PlayFromStart)
    (:Update
      ;[1 1 1] Animate attack
      (Transformation|SetActorLocation (Variables|Default|GetOwningUnit) (Math|Vector|MakeVector (Math|Float|Lerp _x (.x (Variables|Default|GetTargetPoint)) _progression) (Math|Float|Lerp _y (.y (Variables|Default|GetTargetPoint)) _progression) (.z (Transformation|GetActorLocation (Variables|Default|GetOwningUnit)))) false false)
      (Default|SetSprite (Variables|Default|GetOwningUnit) "NewEnumerator2" (.Yaw (Math|Rotator|BreakRotator (Math|Rotator|FindLookatRotation _location_2 _location)))))
    (:Finished
      ;[1 1 1] End Attack
      (Default|SetSprite _owningunit_2 "NewEnumerator0" 9e+01)
      (Variables|Default|SetbAnimating false)
      (Utilities|DelayWhile (Utilities|IsValid (Variables|Default|GetCombatInstance))
        (:Continue
          (if (not (Default|IsAIControlled _owningunit_2))
            (Variables|/Game/Core/GridCombat/Units/BP_Unit.BP_Unit_C|SetbMovementLocked (Variables|Default|GetOwningUnit) (> (Variables|/Game/Core/GridCombat/Units/BP_Unit.BP_Unit_C|GetMovementUsed (Variables|Default|GetOwningUnit)) 0))
            (Default|EndUnitAction _unitcontroller)
            (bind _asbp_player_unit_controller (Utilities|Casting|CastToBP_PlayerUnitController _unitcontroller)
              (:then
                (Default|SaveUnitState _asbp_player_unit_controller))
              (:CastFailed
                _))
            (Class|BPIAbilityInteraction|EndExecution(Message) self)
            (else
              (Class|BPIAbilityInteraction|EndExecution(Message) self))))))
    (:Event
      ;[1 1 1] Attack
      (CallFunction|PerformAbility))))

(event EventCancelAbility
  (|CallParentFunction)
  (Actor|DestroyActor))

(event EventExecuteAbility
  (params (Target :type F%20Grid%20Index%20Structure))
  (|CallParentFunction Target)
  (if (and (Utilities|IsValid (.unit (Default|GetIndexAttributes (Variables|Default|GetGridManagerRef) Target))) (CallFunction|IsValidIndex Target))
    ;[1 1 1] Stamina Cost
    (Class|BPIStamina|UseStamina(Message) (Variables|Default|GetOwningUnit) (CallFunction|GetStaminaCost) true)
    (Variables|/Game/Core/GridCombat/Units/BP_Unit.BP_Unit_C|SetbUsedAction (Variables|Default|GetOwningUnit) true)
    (bind _returnvalue (Game|SpawnActorfromClass "/Game/Core/GridCombat/BP_CombatInstance.BP_CombatInstance_C" (Math|Transform|MakeTransform "0, 0, 0" "0, 0, 0" "1,1,1") "AlwaysSpawn" 0 self Target 0))
    (bind _output_get (Variables|Default|SetCombatInstance _returnvalue))
    (Default|EnterCombat _output_get)
    (else
      (CallFunction|CancelAbility))))

(fn ConstructionScript
  (|CallParentFunction))

(fn ShowBattleForecast
  (params (Target :type BP%20Unit%20Object%20Reference))
  (Development|PrintString (Utilities|String|ToString(Integer) (CallFunction|CalculatePower Target))))

(fn GetIndexesinRange
  (params (StartIndex :type F%20Grid%20Index%20Structure))
  (return (Default|GetIndexesinAttackRange (Variables|Default|GetOwningUnit) (Variables|Default|GetWeapon) StartIndex)))