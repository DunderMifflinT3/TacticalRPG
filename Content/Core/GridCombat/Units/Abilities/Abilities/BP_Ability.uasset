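; BP_Ability is an ability actor for grid combat units, handling activation, cancel, execution and cleanup through the turn manager.
; Activation finds tiles in range, highlighted for player units, and a range pattern expands the target tile into affected tiles.
; Power, hit and crit derive from unit, weapon and target stats into a target map, which PerformAbility rolls against to deal damage.
; Stamina cost, including inventory weight, and cooldowns gate use.
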(event EventActivateAbility
  (Variables|/Game/Core/GridCombat/BP_TurnManager.BP_TurnManager_C|SetActiveAbility (Variables|/Game/Core/GridCombat/BP_GridManager.BP_GridManager_C|GetTurnManagerRef (Variables|Default|GetGridManagerRef)) self)
  (Variables|Range|SetIndexesInRange (CallFunction|GetIndexesinRange (Variables|/Game/Core/GridCombat/BP_GridActor.BP_GridActor_C|GetGridIndex (Variables|Default|GetOwningUnit))))
  (if (not (Default|IsAIControlled (Variables|Default|GetOwningUnit)))
    (Class|BPIAbilityInteraction|PlayerActivate(Message) self)))

(event EventExecuteAbility
  (params (Target :type F%20Grid%20Index%20Structure))
  (Default|RemoveHighlightedTiles (Variables|Default|GetGridManagerRef) (Variables|Default|GetHighlightType))
  (Default|PantoActor (Variables|/Game/Core/GridCombat/BP_GridManager.BP_GridManager_C|GetGridCamera (Variables|Default|GetGridManagerRef)) (Variables|Default|GetOwningUnit)))

(event EventEndExecution
  (Default|AddAbilityCooldown (Variables|Default|GetOwningUnit) self)
  (Variables|/Game/Core/GridCombat/BP_TurnManager.BP_TurnManager_C|SetActiveAbility (Variables|/Game/Core/GridCombat/BP_GridManager.BP_GridManager_C|GetTurnManagerRef (Variables|Default|GetGridManagerRef)) 0)
  (Actor|DestroyActor))

(event EventOnHover
  (params (Index :type F%20Grid%20Index%20Structure)))

(event EventAnimateAbility
  (params (Target :type F%20Grid%20Index%20Structure))
  (bind _asplayer_controller_grid (Utilities|Casting|CastToPlayerController_Grid (Game|GetPlayerController 0)))
  (Default|ToggleInput _asplayer_controller_grid false)
  (Variables|Default|SetbAnimating true))

(event EventCancelAbility
  (Default|ShowUnitActions (Variables|/Game/Core/GridCombat/Units/BP_Unit.BP_Unit_C|GetUnitController (Variables|Default|GetOwningUnit)))
  (Default|RemoveHighlightedTiles (Variables|Default|GetGridManagerRef) (Variables|Default|GetHighlightType))
  (Default|PantoActor (Variables|/Game/Core/GridCombat/BP_GridManager.BP_GridManager_C|GetGridCamera (Variables|Default|GetGridManagerRef)) (Variables|Default|GetOwningUnit)))

(event EventPlayerActivate
  (Default|HighlightTiles (Variables|Default|GetGridManagerRef) (Variables|Range|GetIndexesInRange) (Variables|Default|GetHighlightType)))

(fn ConstructionScript
  (Variables|Default|SetGridManagerRef (Variables|/Game/Core/GridCombat/BP_GridActor.BP_GridActor_C|GetGridManagerRef (Variables|Default|GetOwningUnit)))
  (Variables|Combat|SetWeapon (.Weapon (Default|GetMainWeapon (Variables|/Game/Core/GridCombat/Units/BP_Unit.BP_Unit_C|GetInventoryComponent (Variables|Default|GetOwningUnit))))))

(fn GetIndexesinRange
  (params (StartIndex :type F%20Grid%20Index%20Structure))
  (return (Default|GetIndexesinRange (Variables|Default|GetGridManagerRef) StartIndex (Variables|Range|GetMinRange) (Variables|Range|GetMaxRange) (Variables|Range|GetVerticalRange) false)))

(fn GetConnectedIndexes
  (params (UnitIndex :type F%20Grid%20Index%20Structure) (TargetIndex :type F%20Grid%20Index%20Structure))
  (switch Utilities|FlowControl|Switch|SwitchonERangePattern (Variables|Range|GetRangePattern)
    (:NewEnumerator5
      (return (Utilities|Array|MakeArray TargetIndex)))
    (:NewEnumerator0
      (return (Default|GetIndexesinRange (Variables|Default|GetGridManagerRef) TargetIndex 0 (Variables|Range|GetPatternRange) (Variables|Range|GetVerticalRange) false)))
    (:NewEnumerator1
      (return (Default|GetIndexesinRange (Variables|Default|GetGridManagerRef) TargetIndex 0 (Variables|Range|GetPatternRange) (Variables|Range|GetVerticalRange) true)))
    (:NewEnumerator2
      (return (Default|GetLineinDirection (Variables|Default|GetGridManagerRef) TargetIndex (Default|GetDirectionOfIndex (Variables|Default|GetGridManagerRef) UnitIndex TargetIndex) (Variables|Range|GetPatternRange) (Variables|Range|GetVerticalRange))))
    (:NewEnumerator6
      (return (Default|GetHorizontalLineinDirection (Variables|Default|GetGridManagerRef) TargetIndex (Default|GetDirectionOfIndex (Variables|Default|GetGridManagerRef) UnitIndex TargetIndex) (Variables|Range|GetPatternRange) (Variables|Range|GetVerticalRange))))
    (:NewEnumerator3
      (return (Default|GetIndexesinCross (Variables|Default|GetGridManagerRef) TargetIndex (Variables|Range|GetPatternRange) (Variables|Range|GetVerticalRange))))
    (:NewEnumerator4
      (return (Default|GetConeinDirection (Variables|Default|GetGridManagerRef) TargetIndex (Default|GetDirectionOfIndex (Variables|Default|GetGridManagerRef) UnitIndex TargetIndex) (Variables|Range|GetPatternRange) (Variables|Range|GetVerticalRange))))))

(fn IsValidIndex
  (params (Index :type F%20Grid%20Index%20Structure))
  (return (Utilities|Array|ContainsItem (Variables|Range|GetIndexesInRange) Index)))

(fn CalculatePower
  (params (Target :type BP%20Unit%20Object%20Reference))
  (Utilities|IsValid Target
    (:Is%20Valid
      (return (Math|Float|Truncate (* (Math|Integer|Max(Integer) (- (+ (Default|GetAttack (Variables|Default|GetOwningUnit) (Variables|Combat|GetWeapon)) (Default|GetInitiationStatModifier (Variables|Default|GetOwningUnit) (Variables|/Game/Core/GridCombat/Units/Equipment/Weapons/BP_Weapon.BP_Weapon_C|GetAttackStat (Variables|Combat|GetWeapon))) (Variables|Combat|GetBasePower)) (+ (Default|GetGuard Target (Variables|Combat|GetWeapon)) (Default|GetCounterStatModifier Target (Variables|/Game/Core/GridCombat/Units/Equipment/Weapons/BP_Weapon.BP_Weapon_C|GetDefendStat (Variables|Combat|GetWeapon)))))) (Default|GetDamageModifier Target (CallFunction|GetDamageType))))))
    (:Is%20Not%20Valid
      (return 0))))

(fn CalculateHit
  (params (Target :type BP%20Unit%20Object%20Reference))
  (Utilities|IsValid Target
    (:Is%20Valid
      (return (Math|Integer|Max(Integer) (- (+ (Default|GetAccuracy (Variables|Default|GetOwningUnit) (Variables|Combat|GetWeapon)) (Variables|Combat|GetBaseAccuracy)) (Default|GetEvasion Target)))))
    (:Is%20Not%20Valid
      (return 100))))

(fn CalculateCritical
  (params (Target :type BP%20Unit%20Object%20Reference))
  (Utilities|IsValid Target
    (:Is%20Valid
      (if (and (Variables|Combat|GetbCanCrit) (Utilities|Enum|Equal(Enum) (Variables|Range|GetRangePattern) "NewEnumerator5"))
        (return (- (+ (Default|GetCritical (Variables|Default|GetOwningUnit) (Variables|Combat|GetWeapon)) (Variables|Combat|GetBaseCritical)) (Default|GetCriticalAvoid Target)))
        (else
          (return 0))))
    (:Is%20Not%20Valid
      (return 0))))

(fn GetCriticalModifier
  (return (Variables|Combat|GetCriticalModifier)))

(fn GetStaminaCost
  (return (+ (Variables|Combat|GetBaseStaminaCost) (Default|GetInventoryWeight (Variables|/Game/Core/GridCombat/Units/BP_Unit.BP_Unit_C|GetInventoryComponent (Variables|Default|GetOwningUnit))))))

(fn GetDamageType
  (if (Utilities|Enum|Equal(Enum) (Variables|Combat|GetDamageType) "NewEnumerator0")
    (return (Variables|/Game/Core/GridCombat/Units/Equipment/Weapons/BP_Weapon.BP_Weapon_C|GetDamageType (Variables|Combat|GetWeapon)))
    (else
      (return (Variables|Combat|GetDamageType)))))

(fn CanActivate
  (bind _owningunit (Variables|Default|GetOwningUnit))
  (return (and (>= (Variables|/Game/Core/GridCombat/Units/UnitComponents/BP_StaminaComponent.BP_StaminaComponent_C|GetCurrentStamina (Variables|/Game/Core/GridCombat/Units/BP_Unit.BP_Unit_C|GetStaminaComponent _owningunit)) (CallFunction|GetStaminaCost)) (not (.ReturnValue (Utilities|Map|Find (Variables|/Game/Core/GridCombat/Units/BP_Unit.BP_Unit_C|GetCooldowns _owningunit) (Utilities|GetClass self)))))))

(fn AddtoTargetMap
  (params (Target :type BP%20Unit%20Object%20Reference))
  (Utilities|Map|Add (Variables|Combat|GetTargetMap) Target (Utilities|Struct|MakeFDamage (CallFunction|CalculatePower Target) (CallFunction|CalculateHit Target) (CallFunction|CalculateCritical Target))))

(fn PerformAbility
  (bind _keys (Utilities|Map|Keys (Variables|Combat|GetTargetMap)))
  (for _array_element _keys
    ;[1 1 1] Determines if the ability hit this target
    (if (<= (Math|Random|RandomIntegerinRange 1 100) (.hit (.Value (Utilities|Map|Find (Variables|Combat|GetTargetMap) _array_element))))
      ;[1 1 1] Determines if the ability is a critical hit
      (if (<= (Math|Random|RandomIntegerinRange 1 100) (.critical (.Value (Utilities|Map|Find (Variables|Combat|GetTargetMap) _array_element))))
        (Development|PrintString "Critical!")
        (Class|BPIHealth|TakeDamage(Message) _array_element (Math|Float|Truncate (* (.power (.Value (Utilities|Map|Find (Variables|Combat|GetTargetMap) _array_element))) (CallFunction|GetCriticalModifier))) (CallFunction|GetDamageType) true)
        (else
          (Class|BPIHealth|TakeDamage(Message) _array_element (.power (.Value (Utilities|Map|Find (Variables|Combat|GetTargetMap) _array_element))) (CallFunction|GetDamageType) true)))
      (else
        (Development|PrintString "Miss")))))