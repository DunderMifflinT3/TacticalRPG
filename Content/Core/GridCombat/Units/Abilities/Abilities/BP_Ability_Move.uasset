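; Movement ability for grid combat units that pathfinds to the target tile, records the path cost as movement used, and cancels if no path exists.
; A timeline moves the unit along the generated path spline at constant speed while the camera follows.
; Grounded units trace down for height; flying units rise to the path's highest point, travel level, then descend.
; On finish, execution ends, reshowing unit actions for player-controlled units.
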(event EventCancelAbility
  (|CallParentFunction)
  (Actor|DestroyActor))

(event EventExecuteAbility
  (params (Target :type F%20Grid%20Index%20Structure))
  (bind _owningunit (Variables|Default|GetOwningUnit))
  (bind _gridmanagerref (Variables|Default|GetGridManagerRef))
  (bind _gridindex (Variables|/Game/Core/GridCombat/BP_GridActor.BP_GridActor_C|GetGridIndex _owningunit))
  (bind (_path _pathcost _bpathfound) (Default|FindPathtoIndex _gridmanagerref _owningunit _gridindex Target))
  (|CallParentFunction Target)
  (if _bpathfound
    (Variables|/Game/Core/GridCombat/Units/BP_Unit.BP_Unit_C|SetMovementUsed (Variables|Default|GetOwningUnit) _pathcost)
    (Default|GenerateSplinePath (Variables|Default|GetGridManagerRef) _path)
    (Class|BPIAbilityInteraction|AnimateAbility(Message) self Target)
    (else
      (CallFunction|CancelAbility))))

(event EventAnimateAbility
  (params (Target :type F%20Grid%20Index%20Structure))
  (bind _gridmanagerref (Variables|Default|GetGridManagerRef))
  (bind _gridmanagerref_2 (Variables|Default|GetGridManagerRef))
  (bind _owningunit (Variables|Default|GetOwningUnit))
  (bind _gridmanagerref_3 (Variables|Default|GetGridManagerRef))
  (bind _owningunit_2 (Variables|Default|GetOwningUnit))
  (bind _owningunit_3 (Variables|Default|GetOwningUnit))
  (bind _returnvalue (Transformation|GetActorLocation _owningunit_3))
  (bind _returnvalue_2 (Transformation|GetActorLocation _owningunit_2))
  (bind _gridui (Variables|/Game/Core/GridCombat/BP_GridManager.BP_GridManager_C|GetGridUI _gridmanagerref))
  (bind _gridmap (Variables|/Game/Core/GridCombat/BP_GridManager.BP_GridManager_C|GetGridMap _gridmanagerref_2))
  (bind _gridindex (Variables|/Game/Core/GridCombat/BP_GridActor.BP_GridActor_C|GetGridIndex _owningunit))
  (bind _gridui_2 (Variables|/Game/Core/GridCombat/BP_GridManager.BP_GridManager_C|GetGridUI _gridmanagerref_3))
  (bind _value (Utilities|Map|Find _gridmap _gridindex))
  (bind _pathspline (Variables|/Game/Core/GridCombat/BP_GridUI.BP_GridUI_C|GetPathSpline _gridui))
  (bind _pathspline_2 (Variables|/Game/Core/GridCombat/BP_GridUI.BP_GridUI_C|GetPathSpline _gridui_2))
  (bind _returnvalue_3 (Spline|GetSplineLength _pathspline_2))
  (bind _returnvalue_4 (Spline|GetSplineLength _pathspline))
  (bind (_x _y _z) (Math|Vector|BreakVector (.location _value)))
  (|CallParentFunction Target)
  (Variables|/Game/Core/GridCombat/BP_GridCamera.BP_GridCamera_C|SetFollowActor (Variables|/Game/Core/GridCombat/BP_GridManager.BP_GridManager_C|GetGridCamera _gridmanagerref) (Variables|Default|GetOwningUnit))
  (Variables|Default|SetStartLocation (Transformation|GetActorLocation (Variables|Default|GetOwningUnit)))
  (if (not (<= (Spline|GetNumberOfSplinePoints _pathspline) 1))
    (if (not (Variables|/Game/Core/GridCombat/Units/BP_Unit.BP_Unit_C|GetbFlying (Variables|Default|GetOwningUnit)))
      ;[1 1 1] Sets play rate according to the length of the path. Makes speed of movement constant
      (Components|Timeline|SetPlayRate (Variables|Default|GetTL_GroundedMove) (* (/ 1.0 (Math|Conversions|ToFloat(Integer) (Spline|GetNumberOfSplinePoints _pathspline))) (Variables|/Game/Core/GridCombat/Units/BP_Unit.BP_Unit_C|GetMoveSpeed (Variables|Default|GetOwningUnit))))
      (bind _progression (Timeline|TL_GroundedMove PlayFromStart)
        (:Update
          ;[1 1 1] Grounded Movement
          (bind _outhit (Collision|LineTraceByChannel (Math|Vector|MakeVector (.x (Spline|GetLocationatDistanceAlongSpline _pathspline (* _progression _returnvalue_4) "World")) (.y (Spline|GetLocationatDistanceAlongSpline _pathspline (* _progression _returnvalue_4) "World")) 1e+03) (Math|Vector|MakeVector (.x (Spline|GetLocationatDistanceAlongSpline _pathspline (* _progression _returnvalue_4) "World")) (.y (Spline|GetLocationatDistanceAlongSpline _pathspline (* _progression _returnvalue_4) "World")) -1e+01) "TraceTypeQuery1" false 0 "None"))
          (Transformation|SetActorLocation (Variables|Default|GetOwningUnit) (Math|Vector|MakeVector (.x (Spline|GetLocationatDistanceAlongSpline _pathspline (* _progression _returnvalue_4) "World")) (.y (Spline|GetLocationatDistanceAlongSpline _pathspline (* _progression _returnvalue_4) "World")) (.z (.location _outhit))) false false)
          ;[1 1 1] Prevents strange error where head socket briefly appears in the wrong place
          (if (Math|Float|NearlyEqual(Float) (* _progression _returnvalue_4) _returnvalue_4 1.0)
            (Default|SetSprite (Variables|Default|GetOwningUnit) "NewEnumerator1" 9e+01)
            (else
              (Default|SetSprite (Variables|Default|GetOwningUnit) "NewEnumerator1" (.yaw (Spline|GetRotationatDistanceAlongSpline _pathspline (* _progression _returnvalue_4) "World")))))
          (Default|UpdateGridIndex (Variables|Default|GetOwningUnit)))
        (:Finished
          (Default|SetSprite (Variables|Default|GetOwningUnit) "NewEnumerator1" 9e+01 :!label _label)
          (Variables|/Game/Core/GridCombat/BP_GridCamera.BP_GridCamera_C|SetFollowActor (Variables|/Game/Core/GridCombat/BP_GridManager.BP_GridManager_C|GetGridCamera (Variables|Default|GetGridManagerRef)) 0)
          (if (Default|IsAIControlled (Variables|Default|GetOwningUnit))
            (Class|BPIAbilityInteraction|EndExecution(Message) self)
            (else
              (Default|ShowUnitActions (Variables|/Game/Core/GridCombat/Units/BP_Unit.BP_Unit_C|GetUnitController (Variables|Default|GetOwningUnit)))
              (Class|BPIAbilityInteraction|EndExecution(Message) self)))))
      (else
        (bind _output_get (Variables|Default|SetTargetHeight (Default|GetMaxZCoordonPath (Variables|/Game/Core/GridCombat/BP_GridManager.BP_GridManager_C|GetGridUI (Variables|Default|GetGridManagerRef)))))
        (if (> _output_get (.z _returnvalue_2))
          (Components|Timeline|SetPlayRate (Variables|Default|GetTL_Hover) (* (/ 1.0 (/ (- _output_get (.z _returnvalue_2)) (Variables|/Game/Core/GridCombat/BP_GridManager.BP_GridManager_C|GetTileHeight (Variables|Default|GetGridManagerRef)))) (Variables|/Game/Core/GridCombat/Units/BP_Unit.BP_Unit_C|GetMoveSpeed (Variables|Default|GetOwningUnit)) 2.0))
          (bind _progression_2 (Timeline|TL_Hover PlayFromStart)
            (:Update
              ;[1 1 1] Unit hovers to the Z coordinate of the highest path node
              (Transformation|SetActorLocation (Variables|Default|GetOwningUnit) (Math|Vector|MakeVector (.x (Variables|Default|GetStartLocation)) (.y (Variables|Default|GetStartLocation)) (Math|Float|Lerp (.z (Variables|Default|GetStartLocation)) (Variables|Default|GetTargetHeight) _progression_2)) false false))
            (:Finished
              (Components|Timeline|SetPlayRate (Variables|Default|GetTL_FlyingMove) (* (/ 1.0 (Math|Conversions|ToFloat(Integer) (Spline|GetNumberOfSplinePoints _pathspline_2))) (Variables|/Game/Core/GridCombat/Units/BP_Unit.BP_Unit_C|GetMoveSpeed (Variables|Default|GetOwningUnit))) :!label _label_2)
              (bind _progression_3 (Timeline|TL_FlyingMove PlayFromStart)
                (:Update
                  ;[1 1 1] Flying Movement
                  (Transformation|SetActorLocation (Variables|Default|GetOwningUnit) (Math|Vector|MakeVector (.x (Spline|GetLocationatDistanceAlongSpline _pathspline_2 (* _progression_3 _returnvalue_3) "World")) (.y (Spline|GetLocationatDistanceAlongSpline _pathspline_2 (* _progression_3 _returnvalue_3) "World")) (Variables|Default|GetTargetHeight)) false false)
                  ;[1 1 1] Prevents strange error where head socket briefly appears in the wrong place
                  (if (Math|Float|NearlyEqual(Float) _returnvalue_3 (* _progression_3 _returnvalue_3) 1.0)
                    (Default|SetSprite (Variables|Default|GetOwningUnit) "NewEnumerator1" 9e+01)
                    (else
                      (Default|SetSprite (Variables|Default|GetOwningUnit) "NewEnumerator1" (.yaw (Spline|GetRotationatDistanceAlongSpline _pathspline_2 (* _progression_3 _returnvalue_3) "World")))))
                  (Default|UpdateGridIndex (Variables|Default|GetOwningUnit)))
                (:Finished
                  (if (> (.z _returnvalue) _z)
                    (Components|Timeline|SetPlayRate (Variables|Default|GetTL_Descend) (* (/ 1.0 (/ (- (.z _returnvalue) _z) (Variables|/Game/Core/GridCombat/BP_GridManager.BP_GridManager_C|GetTileHeight (Variables|Default|GetGridManagerRef)))) (Variables|/Game/Core/GridCombat/Units/BP_Unit.BP_Unit_C|GetMoveSpeed (Variables|Default|GetOwningUnit)) 2.0))
                    (bind _progression_4 (Timeline|TL_Descend PlayFromStart)
                      (:Update
                        ;[1 1 1] Unit descends down to the height of the target tile
                        (Transformation|SetActorLocation (Variables|Default|GetOwningUnit) (Math|Vector|MakeVector _x _y (Math|Float|Lerp (Variables|Default|GetTargetHeight) _z _progression_4)) false false))
                      (:Finished
                        (Default|SetSprite (Variables|Default|GetOwningUnit) "NewEnumerator1" 9e+01 :!label _label_3)
                        (Variables|/Game/Core/GridCombat/BP_GridCamera.BP_GridCamera_C|SetFollowActor (Variables|/Game/Core/GridCombat/BP_GridManager.BP_GridManager_C|GetGridCamera (Variables|Default|GetGridManagerRef)) 0)
                        (if (Default|IsAIControlled (Variables|Default|GetOwningUnit))
                          (Class|BPIAbilityInteraction|EndExecution(Message) self)
                          (else
                            (Default|ShowUnitActions (Variables|/Game/Core/GridCombat/Units/BP_Unit.BP_Unit_C|GetUnitController (Variables|Default|GetOwningUnit)))
                            (Class|BPIAbilityInteraction|EndExecution(Message) self)))))
                    (else
                      (goto _label_3)))))))
          (else
            (goto _label_2)))))
    (else
      (goto _label))))

(fn ConstructionScript
  (|CallParentFunction))

(fn GetIndexesinRange
  (params (StartIndex :type F%20Grid%20Index%20Structure))
  (return (Variables|/Game/Core/GridCombat/Units/UnitControllers/BP_UnitController.BP_UnitController_C|GetIndexesInRange (Variables|/Game/Core/GridCombat/Units/BP_Unit.BP_Unit_C|GetUnitController (Variables|Default|GetOwningUnit)))))