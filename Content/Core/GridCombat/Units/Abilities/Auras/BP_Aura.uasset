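; BP_Aura is a grid-combat unit aura that, by default, affects units of the owning unit's faction.
; It registers or unregisters itself on grid indexes within the owner's min, max and vertical range through the grid manager.
; CanBeApplied gates both effect application and per-stat modifier lookups, which return zero for ineligible units.
; The apply and remove effect functions are empty stubs.
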(event Custom|ApplyToUnit
  (params (Unit :type BP%20Unit%20Object%20Reference))
  (if (CallFunction|CanbeApplied Unit)
    (CallFunction|ApplyAuraEffect Unit)))

(event Custom|AddToGrid
  (bind _owningunit (Variables|Default|GetOwningUnit))
  (bind _gridmanagerref (Variables|/Game/Core/GridCombat/BP_GridActor.BP_GridActor_C|GetGridManagerRef _owningunit))
  (for _array_element (Default|GetIndexesinRange _gridmanagerref (Variables|/Game/Core/GridCombat/BP_GridActor.BP_GridActor_C|GetGridIndex _owningunit) (Variables|Default|GetMinRange) (Variables|Default|GetRange) (Variables|Default|GetVerticalRange) false)
    (Default|AddAuratoIndex _gridmanagerref _array_element self)))

(event Custom|RemoveFromGrid
  (bind _owningunit (Variables|Default|GetOwningUnit))
  (bind _gridmanagerref (Variables|/Game/Core/GridCombat/BP_GridActor.BP_GridActor_C|GetGridManagerRef _owningunit))
  (for _array_element (Default|GetIndexesinRange _gridmanagerref (Variables|/Game/Core/GridCombat/BP_GridActor.BP_GridActor_C|GetGridIndex _owningunit) (Variables|Default|GetMinRange) (Variables|Default|GetRange) (Variables|Default|GetVerticalRange) false)
    (Default|RemoveAurafromIndex _gridmanagerref _array_element self)))

(fn ConstructionScript)

(fn CanbeApplied
  (params (Unit :type BP%20Unit%20Object%20Reference))
  (return (Utilities|Enum|Equal(Enum) (Default|GetUnitFaction Unit) (Default|GetUnitFaction (Variables|Default|GetOwningUnit)))))

(fn ApplyAuraEffect
  (params (Unit :type BP%20Unit%20Object%20Reference)))

(fn RemoveAuraEffect)

(fn GetStatModifier
  (params (Unit :type BP%20Unit%20Object%20Reference) (Stat :type EStats%20Enum :default "NewEnumerator9"))
  (if (CallFunction|CanbeApplied Unit)
    (return (.Value (Utilities|Map|Find (Variables|Default|GetStatModifier) Stat)))
    (else
      (return 0))))