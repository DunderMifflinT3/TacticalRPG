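; BP_Passive is the base for unit passive abilities in grid combat.
; Equip and Unequip set and clear the owning unit, while empty event hooks cover turn begin and end, unit or foe initiation, and damage taken or dealt.
; Two getters look up per-stat values in separate initiation and counter modifier maps.
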(event Custom|OnTurnBegin)

(event Custom|OnTurnEnd)

(event EventEquip
  (params (Unit :type BP%20Unit%20Object%20Reference))
  (Variables|Default|SetOwningUnit Unit))

(event EventUnequip
  (Variables|Default|SetOwningUnit 0))

(event EventOnUnitInitiate
  (params (Ability :type BP%20Ability%20Object%20Reference)))

(event EventOnFoeInitiate
  (params (Ability :type BP%20Ability%20Object%20Reference)))

(event EventOnTakeDamage
  (params (Ability :type BP%20Ability%20Object%20Reference)))

(event EventOnDealDamage
  (params (Ability :type BP%20Ability%20Object%20Reference)))

(fn ConstructionScript)

(fn GetInitiationModifier
  (params (Stat :type EStats%20Enum :default "NewEnumerator9"))
  (return (.Value (Utilities|Map|Find (Variables|Default|GetInitiationModifiers) Stat))))

(fn GetCounterModifier
  (params (Stat :type EStats%20Enum :default "NewEnumerator9"))
  (return (.Value (Utilities|Map|Find (Variables|Default|GetCounterModifiers) Stat))))