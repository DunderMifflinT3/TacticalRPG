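; BP_StatusCondition is the base actor for status conditions applied to units in grid combat.
; AddStatusToUnit blocks duplicates of the same class through the unit's StatusComponent, then stores the owner, registers itself and calls ActivateStatus.
; RemoveStatus unregisters from that component and destroys the actor.
; Activation, turn start, turn end and attacked events are empty hooks, presumably for child Blueprints to override.
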(event Custom|Activate%20Status)

(event Custom|AddStatusToUnit
  (params (Unit :type BP%20Unit%20Object%20Reference))
  (if (CallFunction|CanbeApplied Unit)
    (bind _output_get (Variables|Default|SetOwningUnit Unit))
    (Utilities|IsValid (Variables|/Game/Core/GridCombat/Units/BP_Unit.BP_Unit_C|GetStatusComponent _output_get)
      (:Is%20Valid
        (Default|AddStatusCondition (Variables|/Game/Core/GridCombat/Units/BP_Unit.BP_Unit_C|GetStatusComponent _output_get) self)
        (CallFunction|ActivateStatus)))))

(event Custom|Remove%20Status
  (bind _owningunit (Variables|Default|GetOwningUnit))
  (bind _statuscomponent (Variables|/Game/Core/GridCombat/Units/BP_Unit.BP_Unit_C|GetStatusComponent _owningunit))
  (Utilities|IsValid _statuscomponent
    (:Is%20Valid
      (Default|RemoveStatusCondition _statuscomponent self)
      (Actor|DestroyActor))
    (:Is%20Not%20Valid
      (Actor|DestroyActor))))

(event Custom|OnTurnStart)

(event Custom|OnTurnEnd)

(event Custom|OnAttacked
  (params (Ability :type BP%20Ability%20Object%20Reference)))

(fn ConstructionScript)

(fn CanbeApplied
  (params (Unit :type BP%20Unit%20Object%20Reference))
  (if (Default|HasStatus (Variables|/Game/Core/GridCombat/Units/BP_Unit.BP_Unit_C|GetStatusComponent Unit) (Utilities|GetClass self))
    (return false)
    (else
      (return true))))