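; BP_Status_Soaked is a grid-combat unit status condition for being soaked, which cannot be applied to Frozen units.
; At turn start it removes itself unless the unit stands on a wet tile.
; OnAttacked switches on damage type, but its branches are unconnected: ice converting Soaked to Frozen, plus doubled lightning and halved fire damage, both clearing Soaked off wet tiles, never run.
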(event EventOnAttacked
  (params (Ability :type BP%20Ability%20Object%20Reference))
  (switch Utilities|FlowControl|Switch|SwitchonEDamageType (Variables|/Game/Core/GridCombat/Units/Abilities/Abilities/BP_Ability.BP_Ability_C|GetDamageType Ability)))

(event EventOnTurnStart
  (bind _owningunit (Variables|Default|GetOwningUnit))
  ;[1 1 1] Goes away at the start of the unit's turn if they are not standing on a wet tile
  (if (not (Default|IsTileWet (Variables|/Game/Core/GridCombat/BP_GridActor.BP_GridActor_C|GetGridManagerRef _owningunit) (Variables|/Game/Core/GridCombat/BP_GridActor.BP_GridActor_C|GetGridIndex _owningunit)))
    (CallFunction|RemoveStatus)))

(fn ConstructionScript
  (|CallParentFunction))

(fn CanbeApplied
  (params (Unit :type BP%20Unit%20Object%20Reference))
  (if (|CallParentFunction Unit)
    (if (Default|HasStatus (Variables|/Game/Core/GridCombat/Units/BP_Unit.BP_Unit_C|GetStatusComponent Unit) "/Game/Core/GridCombat/Units/StatusConditions/BP_Status_Frozen.BP_Status_Frozen_C")
      (return false)
      (else
        (return true)))
    (else
      (return false))))