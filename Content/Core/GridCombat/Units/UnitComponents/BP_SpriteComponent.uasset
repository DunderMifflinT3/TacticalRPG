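; Unit component for grid combat that drives layered Paper2D flipbook sprites for a unit's head, body and optional mount.
; SetSprite converts Z rotation into one of four directions, then picks flipbooks by action from the stored sprite sets.
; Mounted units use a separate body set plus mount sprites, while unmounted units clear the mount, and Selected reuses the Run animation.
; Setter functions supply the flipbook components and sprite sets.
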(event EventBeginPlay)

(event EventTick
  (params (DeltaSeconds :type Float%20%28single-precision%29)))

(fn SetSprite
  (params (Action :type ESpriteActions%20Enum :default "NewEnumerator0") (ZRotation :type Float%20%28single-precision%29) (Mounted :type Boolean))
  (LocalVariables|SetDirection (Math|Conversions|ToInteger(Byte) (CallFunction|FindSpriteDirection ZRotation)))
  (if (not Mounted)
    (switch Utilities|FlowControl|Switch|SwitchonESpriteActions Action
      (:NewEnumerator0
        ;[1 1 1] Unmounted
        (Sprite|SetFlipbook (Variables|Default|GetHead) (Utilities|Array|Get(acopy) (.idle (Variables|Default|GetHeadSprites)) (LocalVariables|GetDirection)))
        (Sprite|SetFlipbook (Variables|Default|GetBody) (Utilities|Array|Get(acopy) (.idle (Variables|Default|GetBodySprites)) (LocalVariables|GetDirection))))
      (:NewEnumerator1
        (Sprite|SetFlipbook (Variables|Default|GetHead) (Utilities|Array|Get(acopy) (.run (Variables|Default|GetHeadSprites)) (LocalVariables|GetDirection)))
        (Sprite|SetFlipbook (Variables|Default|GetBody) (Utilities|Array|Get(acopy) (.run (Variables|Default|GetBodySprites)) (LocalVariables|GetDirection))))
      (:NewEnumerator2
        (Sprite|SetFlipbook (Variables|Default|GetHead) (Utilities|Array|Get(acopy) (.attack (Variables|Default|GetHeadSprites)) (LocalVariables|GetDirection)))
        (Sprite|SetFlipbook (Variables|Default|GetBody) (Utilities|Array|Get(acopy) (.attack (Variables|Default|GetBodySprites)) (LocalVariables|GetDirection))))
      (:NewEnumerator3
        (Sprite|SetFlipbook (Variables|Default|GetHead) (Utilities|Array|Get(acopy) (.run (Variables|Default|GetHeadSprites)) (LocalVariables|GetDirection)))
        (Sprite|SetFlipbook (Variables|Default|GetBody) (Utilities|Array|Get(acopy) (.run (Variables|Default|GetBodySprites)) (LocalVariables|GetDirection)))))
    (Sprite|SetFlipbook (Variables|Default|GetMount))
    (else
      (switch Utilities|FlowControl|Switch|SwitchonESpriteActions Action
        (:NewEnumerator0
          ;[1 1 1] Mounted
          (Sprite|SetFlipbook (Variables|Default|GetHead) (Utilities|Array|Get(acopy) (.idle (Variables|Default|GetHeadSprites)) (LocalVariables|GetDirection)))
          (Sprite|SetFlipbook (Variables|Default|GetBody) (Utilities|Array|Get(acopy) (.idle (Variables|Default|GetMountedBodySprites)) (LocalVariables|GetDirection)))
          (Sprite|SetFlipbook (Variables|Default|GetMount) (Utilities|Array|Get(acopy) (.idle (Variables|Default|GetMountSprites)) (LocalVariables|GetDirection))))
        (:NewEnumerator1
          (Sprite|SetFlipbook (Variables|Default|GetHead) (Utilities|Array|Get(acopy) (.run (Variables|Default|GetHeadSprites)) (LocalVariables|GetDirection)))
          (Sprite|SetFlipbook (Variables|Default|GetBody) (Utilities|Array|Get(acopy) (.run (Variables|Default|GetMountedBodySprites)) (LocalVariables|GetDirection)))
          (Sprite|SetFlipbook (Variables|Default|GetMount) (Utilities|Array|Get(acopy) (.run (Variables|Default|GetMountSprites)) (LocalVariables|GetDirection))))
        (:NewEnumerator2
          (Sprite|SetFlipbook (Variables|Default|GetHead) (Utilities|Array|Get(acopy) (.attack (Variables|Default|GetHeadSprites)) (LocalVariables|GetDirection)))
          (Sprite|SetFlipbook (Variables|Default|GetBody) (Utilities|Array|Get(acopy) (.attack (Variables|Default|GetMountedBodySprites)) (LocalVariables|GetDirection)))
          (Sprite|SetFlipbook (Variables|Default|GetMount) (Utilities|Array|Get(acopy) (.attack (Variables|Default|GetMountSprites)) (LocalVariables|GetDirection))))
        (:NewEnumerator3
          (Sprite|SetFlipbook (Variables|Default|GetHead) (Utilities|Array|Get(acopy) (.run (Variables|Default|GetHeadSprites)) (LocalVariables|GetDirection)))
          (Sprite|SetFlipbook (Variables|Default|GetBody) (Utilities|Array|Get(acopy) (.run (Variables|Default|GetMountedBodySprites)) (LocalVariables|GetDirection)))
          (Sprite|SetFlipbook (Variables|Default|GetMount) (Utilities|Array|Get(acopy) (.run (Variables|Default|GetMountSprites)) (LocalVariables|GetDirection))))))))

(fn FindSpriteDirection
  (params (ZRotation :type Float%20%28single-precision%29))
  (if (Math|Float|InRange(Float) ZRotation -45.0 45.0)
    (return "NewEnumerator2")
    (elif (Math|Float|InRange(Float) ZRotation 45.0 135.0 false false)
      (return "NewEnumerator1")
      (elif (Math|Float|InRange(Float) ZRotation -135.0 -45.0 false false)
        (return "NewEnumerator0")
        (else
          (return "NewEnumerator3"))))))

(fn SetBodySprites
  (params (Body :type F%20Unit%20Sprites%20Structure) (MountedBody :type F%20Unit%20Sprites%20Structure))
  (Variables|Default|SetBodySprites Body)
  (Variables|Default|SetMountedBodySprites MountedBody))

(fn SetHeadSprites
  (params (Head :type F%20Unit%20Sprites%20Structure))
  (Variables|Default|SetHeadSprites Head))

(fn SetMountSprites
  (params (Mount :type F%20Unit%20Sprites%20Structure))
  (Variables|Default|SetMountSprites Mount))

(fn SetSpriteComponents
  (params (Head :type Paper%20Flipbook%20Component%20Object%20Reference%20%28by%20ref%29) (Body :type Paper%20Flipbook%20Component%20Object%20Reference%20%28by%20ref%29) (Mount :type Paper%20Flipbook%20Component%20Object%20Reference%20%28by%20ref%29))
  (Variables|Default|SetHead Head)
  (Variables|Default|SetBody Body)
  (Variables|Default|SetMount Mount))