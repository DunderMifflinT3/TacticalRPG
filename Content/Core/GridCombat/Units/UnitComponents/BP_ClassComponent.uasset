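; Unit component for grid combat that holds a unit's current class and its per-class levels.
; SetClass looks up the class row in DT_ClassData, caches its stats, movement, weapons, sprites and default AI, and starts unseen classes at level 1.
; Getters expose most of that cached data, and LevelUpClass increments the current class's entry in the ClassLevels map, so earlier class levels persist across class changes.
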(event EventBeginPlay)

(event EventTick
  (params (DeltaSeconds :type Float%20%28single-precision%29)))

(fn SetClass
  (params (ClassName :type Name))
  (bind _output_get (Variables|Default|SetInternalName ClassName))
  (bind _returnvalue (Utilities|GetDataTableRow "/Game/Core/GridCombat/Units/Classes/DT_ClassData.DT_ClassData" _output_get)
    (:then
      (Variables|Default|SetName (.name _returnvalue))
      (Variables|Default|SetDescription (.description _returnvalue))
      (Variables|Default|SetClassType (.classtype _returnvalue))
      (Variables|Default|SetStatModifiers (.statmodifiers _returnvalue))
      (Variables|Default|SetGrowthModifiers (.growthmodifiers _returnvalue))
      (Variables|Default|SetMove (.move _returnvalue))
      (Variables|Default|SetJump (.jump _returnvalue))
      (Variables|Default|SetUsableWeapons (.usableweapons _returnvalue))
      (Variables|Default|SetHeadSprites (.headsprites _returnvalue))
      (Variables|Default|SetBodySprites (.bodysprites _returnvalue))
      (Variables|Default|SetMountedBodySprites (.mountedbodysprites _returnvalue))
      (Variables|Default|SetDefaultAI (.defaultai _returnvalue))
      (if (not (.ReturnValue (Utilities|Map|Find (Variables|Default|GetClassLevels) (Variables|Default|GetInternalName))))
        (Utilities|Map|Add (Variables|Default|GetClassLevels) (Variables|Default|GetInternalName) 1)))))

(fn GetClassType
  (return (Variables|Default|GetClassType)))

(fn GetClassStatModifier
  (params (Stat :type EStats%20Enum :default "NewEnumerator9"))
  (return (.Value (Utilities|Map|Find (Variables|Default|GetStatModifiers) Stat))))

(fn GetClassGrowthModifier
  (params (Stat :type EStats%20Enum :default "NewEnumerator9"))
  (return (.Value (Utilities|Map|Find (Variables|Default|GetGrowthModifiers) Stat))))

(fn GetClassMoveStats
  (return (Variables|Default|GetMove) (Variables|Default|GetJump)))

(fn GetUsableWeapons
  (return (Variables|Default|GetUsableWeapons)))

(fn GetClassSprites
  (return (Variables|Default|GetHeadSprites) (Variables|Default|GetBodySprites) (Variables|Default|GetMountedBodySprites)))

(fn LevelUpClass
  (Utilities|Map|Add (Variables|Default|GetClassLevels) (Variables|Default|GetInternalName) (+ (.Value (Utilities|Map|Find (Variables|Default|GetClassLevels) (Variables|Default|GetInternalName))) 1)))