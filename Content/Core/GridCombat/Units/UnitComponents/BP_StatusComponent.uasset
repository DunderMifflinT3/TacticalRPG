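; Unit component for grid combat that holds the status conditions on its owner.
; Adding stores a status uniquely without consulting its CanBeApplied check, and removal takes it out of the array.
; Turn start, turn end and attacked functions forward the event to every stored status, with the attacking ability passed along.
; HasStatus compares by class but returns on the first element, so later entries are never checked.
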(fn AddStatusCondition
  (params (Status :type BP%20Status%20Condition%20Object%20Reference))
  (Utilities|Array|AddUnique (Variables|Default|GetStatusConditions) Status))

(fn RemoveStatusCondition
  (params (Status :type BP%20Status%20Condition%20Object%20Reference))
  (Utilities|Array|RemoveItem (Variables|Default|GetStatusConditions) Status))

(fn ActivateonTurnStart
  (for _array_element (Variables|Default|GetStatusConditions)
    (Default|OnTurnStart _array_element)))

(fn ActivateonTurnEnd
  (for _array_element (Variables|Default|GetStatusConditions)
    (Default|OnTurnEnd _array_element)))

(fn ActivateonAttacked
  (params (Ability :type BP%20Ability%20Object%20Reference))
  (for _array_element (Variables|Default|GetStatusConditions)
    (Default|OnAttacked _array_element Ability)))

(fn HasStatus
  (params (Status :type BP%20Status%20Condition%20Class%20Reference))
  (for _array_element (Variables|Default|GetStatusConditions)
    (return (== (Utilities|GetClass _array_element) Status)))
  (return false))