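; Inventory component for a grid-combat unit, holding main weapon, second weapon, shield, item and mount slots.
; InitializeInventory spawns item actors from names; adding or removing sends the displaced item to the player inventory in BP_PlayerData.
; Main weapon, shield and mount have equipped flags, gated by CanBeEquipped against the owning BP_Unit.
; Only those equipped items supply stat, combat and growth modifiers, abilities and passives; weight counts just weapon and shield.
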(fn GetEquippedItems
  (if (Variables|Default|GetWeaponEquipped)
    (Utilities|Array|Add (LocalVariables|GetLEquippedItems) (Variables|Default|GetMainWeapon)))
  (if (Variables|Default|GetShieldEquipped)
    (Utilities|Array|Add (LocalVariables|GetLEquippedItems) (Variables|Default|GetShield)))
  (if (Variables|Default|GetMountEquipped)
    (Utilities|Array|Add (LocalVariables|GetLEquippedItems) (Variables|Default|GetMount)))
  (return (LocalVariables|GetLEquippedItems)))

(fn GetMainWeapon
  (return (Variables|Default|GetMainWeapon) (Variables|Default|GetWeaponEquipped)))

(fn GetSecondWeapon
  (return (Variables|Default|GetSecondWeapon)))

(fn GetShield
  (return (Variables|Default|GetShield) (Variables|Default|GetShieldEquipped)))

(fn GetItem
  (params (Slot :type Byte :default 0))
  (return (Variables|Default|GetItem)))

(fn GetMount
  (return (Variables|Default|GetMount) (Variables|Default|GetMountEquipped)))

(fn InitializeInventory
  (params (MainWeapon :type Name) (SecondWeapon :type Name) (Shield :type Name) (Item :type Name) (Mount :type Name))
  (if (Utilities|Name|NotEqual(Name) MainWeapon "None")
    (bind _returnvalue (Game|SpawnActorfromClass "/Game/Core/GridCombat/Units/Equipment/Weapons/BP_Weapon.BP_Weapon_C" (Math|Transform|MakeTransform "0, 0, 0" "0, 0, 0" "1,1,1") "AlwaysSpawn" 0 MainWeapon 0))
    (Management|Add|AddMainWeapon _returnvalue))
  (if (Utilities|Name|NotEqual(Name) SecondWeapon "None")
    (bind _returnvalue_2 (Game|SpawnActorfromClass "/Game/Core/GridCombat/Units/Equipment/Weapons/BP_Weapon.BP_Weapon_C" (Math|Transform|MakeTransform "0, 0, 0" "0, 0, 0" "1,1,1") "AlwaysSpawn" 0 SecondWeapon 0))
    (Management|Add|AddSecondWeapon _returnvalue_2))
  (if (Utilities|Name|NotEqual(Name) Shield "None")
    (bind _returnvalue_3 (Game|SpawnActorfromClass "/Game/Core/GridCombat/Units/Equipment/Weapons/BP_Weapon.BP_Weapon_C" (Math|Transform|MakeTransform "0, 0, 0" "0, 0, 0" "1,1,1") "AlwaysSpawn" 0 Shield 0))
    (Management|Add|AddShield _returnvalue_3))
  (if (Utilities|Name|NotEqual(Name) Item "None")
    (bind _returnvalue_4 (Game|SpawnActorfromClass "/Game/Core/GridCombat/Units/Equipment/BP_Equipment.BP_Equipment_C" (Math|Transform|MakeTransform "0, 0, 0" "0, 0, 0" "1,1,1") "AlwaysSpawn" 0 Item 0))
    (Management|Add|AddItem _returnvalue_4))
  (if (Utilities|Name|NotEqual(Name) Mount "None")
    (bind _returnvalue_5 (Game|SpawnActorfromClass "/Game/Core/GridCombat/Units/Equipment/Mounts/BP_Mount.BP_Mount_C" (Math|Transform|MakeTransform "0, 0, 0" "0, 0, 0" "1,1,1") "AlwaysSpawn" 0 Mount 0))
    (Management|Add|AddMount _returnvalue_5)))

(fn SetUsableWeapons
  (params (UsableWeapons :type Array%20of%20EWeaponType%20Enums :default "NewEnumerator0"))
  (Variables|Default|SetUsableWeapons UsableWeapons))

(fn GetInventoryStatModifier
  (params (Stat :type EStats%20Enum :default "NewEnumerator9"))
  (for _array_element (Retrieval|GetEquippedItems)
    (LocalVariables|SetLModifier (+ (LocalVariables|GetLModifier) (Default|GetStatModifier _array_element Stat))))
  (return (LocalVariables|GetLModifier)))

(fn GetInventoryCombatStatModifier
  (params (Stat :type ECombatStats%20Enum :default "NewEnumerator7"))
  (for _array_element (Retrieval|GetEquippedItems)
    (LocalVariables|SetLModifier (+ (LocalVariables|GetLModifier) (Default|GetCombatStatModifier _array_element Stat))))
  (return (LocalVariables|GetLModifier)))

(fn GetInventoryGrowthModifier
  (params (Stat :type EStats%20Enum :default "NewEnumerator9"))
  (for _array_element (Retrieval|GetEquippedItems)
    (LocalVariables|SetLModifier (+ (LocalVariables|GetLModifier) (Default|GetGrowthModifier _array_element Stat))))
  (return (LocalVariables|GetLModifier)))

(fn GetInventoryWeight
  (if (Variables|Default|GetWeaponEquipped)
    (LocalVariables|SetLWeight (Variables|/Game/Core/GridCombat/Units/Equipment/Weapons/BP_Weapon.BP_Weapon_C|GetWeight (Variables|Default|GetMainWeapon))))
  (if (Variables|Default|GetShieldEquipped)
    (LocalVariables|SetLWeight (+ (LocalVariables|GetLWeight) (Variables|/Game/Core/GridCombat/Units/Equipment/Weapons/BP_Weapon.BP_Weapon_C|GetWeight (Variables|Default|GetShield)))))
  (return (LocalVariables|GetLWeight)))

(fn SwapWeapons
  (LocalVariables|SetLTempWeapon (Variables|Default|GetMainWeapon))
  (Variables|Default|SetMainWeapon (Variables|Default|GetSecondWeapon))
  (Variables|Default|SetSecondWeapon (LocalVariables|GetLTempWeapon)))

(fn GetInventoryAbilities
  (for _array_element (Retrieval|GetEquippedItems)
    (for _array_element_2 (Variables|/Game/Core/GridCombat/Units/Equipment/BP_Equipment.BP_Equipment_C|GetAbilities _array_element)
      (Utilities|Array|Add (LocalVariables|GetLAbilities) _array_element_2)))
  (return (LocalVariables|GetLAbilities)))

(fn GetInventoryPassives
  (for _array_element (Retrieval|GetEquippedItems)
    (for _array_element_2 (Variables|/Game/Core/GridCombat/Units/Equipment/BP_Equipment.BP_Equipment_C|GetPassives _array_element)
      (Utilities|Array|Add (LocalVariables|GetLPassives) _array_element_2)))
  (return (LocalVariables|GetLPassives)))

(fn ToggleWeaponEquipped
  (params (Equipped :type Boolean))
  (if Equipped
    (Variables|Default|SetWeaponEquipped (Default|CanbeEquipped (Variables|Default|GetMainWeapon) (.AsBP%20Unit (Utilities|Casting|CastToBP_Unit (Components|GetOwner)))))
    (else
      (Variables|Default|SetWeaponEquipped false))))

(fn ToggleShieldEquipped
  (params (Equipped :type Boolean))
  (if Equipped
    (Variables|Default|SetShieldEquipped (Default|CanbeEquipped (Variables|Default|GetShield) (.AsBP%20Unit (Utilities|Casting|CastToBP_Unit (Components|GetOwner)))))
    (else
      (Variables|Default|SetShieldEquipped false))))

(fn ToggleMounted
  (params (Mounted :type Boolean))
  (if Mounted
    (Variables|Default|SetMountEquipped (Default|CanbeEquipped (Variables|Default|GetMount) (.AsBP%20Unit (Utilities|Casting|CastToBP_Unit (Components|GetOwner)))))
    (else
      (Variables|Default|SetMountEquipped false))))

(fn AddMainWeapon
  (params (Weapon :type BP%20Weapon%20Object%20Reference))
  (Utilities|IsValid (Variables|Default|GetMainWeapon)
    (:Is%20Valid
      (Management|Remove|RemoveMainWeapon))
    (:Is%20Not%20Valid
      _))
  (Variables|Default|SetMainWeapon Weapon)
  (Equipping|ToggleWeaponEquipped true))

(fn RemoveMainWeapon
  (Management|SendtoPlayerInventory (Variables|Default|GetMainWeapon))
  (Variables|Default|SetMainWeapon 0)
  (Equipping|ToggleWeaponEquipped false))

(fn AddSecondWeapon
  (params (Weapon :type BP%20Weapon%20Object%20Reference))
  (Utilities|IsValid (Variables|Default|GetSecondWeapon)
    (:Is%20Valid
      (Management|Remove|RemoveSecondWeapon))
    (:Is%20Not%20Valid
      _))
  (Variables|Default|SetSecondWeapon Weapon))

(fn RemoveSecondWeapon
  (Management|SendtoPlayerInventory (Variables|Default|GetSecondWeapon))
  (Variables|Default|SetSecondWeapon 0))

(fn SendtoPlayerInventory
  (params (Item :type BP%20Equipment%20Object%20Reference))
  (bind _returnvalue (Actor|GetActorOfClass "/Game/Core/GridCombat/BP_PlayerData.BP_PlayerData_C"))
  (Default|AddtoPlayerInventory _returnvalue (Variables|Default|GetItem)))

(fn AddShield
  (params (Shield :type BP%20Weapon%20Object%20Reference))
  (Utilities|IsValid (Variables|Default|GetShield)
    (:Is%20Valid
      (Management|Remove|RemoveShield))
    (:Is%20Not%20Valid
      _))
  (Variables|Default|SetShield Shield)
  (Equipping|ToggleShieldEquipped true))

(fn RemoveShield
  (Management|SendtoPlayerInventory (Variables|Default|GetShield))
  (Variables|Default|SetShield 0)
  (Equipping|ToggleShieldEquipped false))

(fn AddItem
  (params (Item :type BP%20Equipment%20Object%20Reference))
  (Utilities|IsValid (Variables|Default|GetItem)
    (:Is%20Valid
      (Management|Remove|RemoveItem))
    (:Is%20Not%20Valid
      _))
  (Variables|Default|SetItem Item))

(fn RemoveItem
  (Management|SendtoPlayerInventory (Variables|Default|GetItem))
  (Variables|Default|SetItem 0))

(fn AddMount
  (params (Mount :type BP%20Mount%20Object%20Reference))
  (Utilities|IsValid (Variables|Default|GetMount)
    (:Is%20Valid
      (Management|Remove|RemoveMount))
    (:Is%20Not%20Valid
      _))
  (Variables|Default|SetMount Mount)
  (Equipping|ToggleMounted true))

(fn RemoveMount
  (Management|SendtoPlayerInventory (Variables|Default|GetMount))
  (Variables|Default|SetMount 0)
  (Equipping|ToggleMounted false))