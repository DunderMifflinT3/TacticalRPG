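; Stamina component for grid combat units that tracks current and maximum stamina.
; UseStamina clamps at zero and notifies the owner with an exhaust message when Exhaust is set, otherwise it never drains stamina below one.
; RestoreStamina adds stamina up to the maximum.
; UpdateMaxStamina shifts current stamina by the change in maximum, with a floor of one, then stores the new maximum.
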(event Custom|UseStamina
  (params (Stamina :type Integer) (Exhaust :type Boolean))
  (bind _returnvalue (Math|Integer|Max(Integer) Stamina))
  (if Exhaust
    (Variables|Default|SetCurrentStamina (Math|Integer|Max(Integer) (- (Variables|Default|GetCurrentStamina) _returnvalue)))
    (if (<= (Variables|Default|GetCurrentStamina) 0)
      (Class|BPIStamina|Exhaust(Message) (Components|GetOwner)))
    (else
      (Variables|Default|SetCurrentStamina (Math|Integer|Max(Integer) (- (Variables|Default|GetCurrentStamina) _returnvalue) 1)))))

(event Custom|RestoreStamina
  (params (Amount :type Integer))
  (Variables|Default|SetCurrentStamina (Math|Integer|Min(Integer) (+ (Variables|Default|GetCurrentStamina) (Math|Integer|Max(Integer) Amount)) (Variables|Default|GetMaxStamina))))

(fn UpdateMaxStamina
  (params (MaxStamina :type Integer))
  (Variables|Default|SetCurrentStamina (Math|Integer|Max(Integer) (+ (Variables|Default|GetCurrentStamina) (- MaxStamina (Variables|Default|GetMaxStamina))) 1))
  (Variables|Default|SetMaxStamina MaxStamina))