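; BP_HealthComponent is a unit component for grid combat that tracks a unit's current and maximum HP.
; Damage and healing ignore negative amounts; non-lethal damage stops at one HP, while lethal damage reaching zero sends a death message to the owner.
; Changing max health shifts current HP by the same difference without dropping it below one.
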(event Custom|TakeDamage
  (params (Damage :type Integer) (Lethal :type Boolean))
  (bind _returnvalue (Math|Integer|Max(Integer) Damage))
  (if Lethal
    (Variables|Default|SetCurrentHP (Math|Integer|Max(Integer) (- (Variables|Default|GetCurrentHP) _returnvalue)))
    (if (<= (Variables|Default|GetCurrentHP) 0)
      (Class|BPIHealth|Death(Message) (Components|GetOwner)))
    (else
      (Variables|Default|SetCurrentHP (Math|Integer|Max(Integer) (- (Variables|Default|GetCurrentHP) _returnvalue) 1)))))

(event Custom|RestoreHealth
  (params (HealAmount :type Integer))
  (Variables|Default|SetCurrentHP (Math|Integer|Min(Integer) (+ (Variables|Default|GetCurrentHP) (Math|Integer|Max(Integer) HealAmount)) (Variables|Default|GetMaxHP))))

(fn UpdateMaxHealth
  (params (MaxHealth :type Integer))
  (Variables|Default|SetCurrentHP (Math|Integer|Max(Integer) (+ (Variables|Default|GetCurrentHP) (- MaxHealth (Variables|Default|GetMaxHP))) 1))
  (Variables|Default|SetMaxHP MaxHealth))