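; Terrain manager actor that builds stepped tile terrain from an array of heightmap textures, one height layer per texture.
; Each white pixel becomes a tile, autotiled by an eight-neighbour bitmask that maps to a Center, Corner, Inner or Edge mesh and rotation.
; Transforms are grouped by type, then batch-added to instanced mesh components.
; The construction script only stores the actor location as offset; its GenerateTerrainHeight call is disconnected.
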(event EventBeginPlay)

(event Collision|EventActorBeginOverlap
  (params (OtherActor :type Actor%20Object%20Reference)))

(event EventTick
  (params (DeltaSeconds :type Float%20%28single-precision%29)))

(fn ConstructionScript
  (Variables|Default|SetTerrainOffset (Transformation|GetActorLocation)))

(fn GetInstancedMeshComponent
  (params (BitmaskValue :type Integer))
  (bind _bitmaskvaluemap (Variables|Default|GetBitmaskValueMap))
  (bind _value (Utilities|Map|Find _bitmaskvaluemap BitmaskValue))
  (return (Utilities|Select :Index _value :Option%200 (Variables|Default|GetCenter) :Option%201 (Variables|Default|GetCorner) :Option%202 (Variables|Default|GetInner) :Option%203 (Variables|Default|GetEdge)) (.Value (Utilities|Map|Find (Variables|Default|GetBitmaskRotationMap) BitmaskValue)) _value))

(fn GenerateTerrainHeight
  (bind _tilesize (Variables|Default|GetTileSize))
  (bind _transforms (Variables|Default|GetTransforms))
  (bind _tilesize_2 (Variables|Default|GetTileSize))
  (if (> (Utilities|Array|Length (Variables|Default|GetHeightmap)) 0)
    (for (_array_element _array_index) (Variables|Default|GetHeightmap)
      (bind (_texturewidth _textureheight _pixelarray) (Class|VictoryBPFunctionLibrary|VictoryGetPixelsArrayfromT2D _array_element))
      (Variables|Default|SetPixelArray _pixelarray)
      (Variables|Default|SetTerrainSize (Utilities|Struct|MakeFGridIndex _texturewidth _textureheight))
      (for _index (range 0 (- (.x (Variables|Default|GetTerrainSize)) 1))
        (for _index_2 (range 0 (- (.y (Variables|Default|GetTerrainSize)) 1))
          (if (== (.FoundColor (Class|VictoryBPFunctionLibrary|VictoryGetPixel (Variables|Default|GetPixelArray) (.y (Variables|Default|GetTerrainSize)) _index _index_2)) "(R=1.000000,G=1.000000,B=1.000000,A=1.000000)")
            (bind _output_get (LocalVariables|SetLTransforms (.transforms (.Value (Utilities|Map|Find _transforms (.NewParam (CallFunction|GetInstancedMeshComponent (CallFunction|GetBitmaskValue _index _index_2))))))))
            (Utilities|Array|Add _output_get (Math|Transform|MakeTransform (+ (Variables|Default|GetTerrainOffset) (Math|Vector|MakeVector (+ (* _index _tilesize_2) (/ _tilesize_2 2.0)) (+ (* _index_2 _tilesize) (/ _tilesize 2.0)) (* _array_index (Variables|Default|GetTileHeight)))) (.Rotation (CallFunction|GetInstancedMeshComponent (CallFunction|GetBitmaskValue _index _index_2)))))
            (Utilities|Map|Add _transforms (.NewParam (CallFunction|GetInstancedMeshComponent (CallFunction|GetBitmaskValue _index _index_2))) (Utilities|Struct|MakeFTerrainTransforms _output_get))))))
    (bind _keys (Utilities|Map|Keys (Variables|Default|GetTransforms)))
    (for _array_element_2 _keys
      (switch int _array_element_2
        (:Default
          (Components|InstancedStaticMesh|AddInstances (Variables|Default|GetCenter) (.transforms (.Value (Utilities|Map|Find (Variables|Default|GetTransforms) _array_element_2))) false :!label _label))
        (:0
          (goto _label))
        (:1
          (Components|InstancedStaticMesh|AddInstances (Variables|Default|GetCorner) (.transforms (.Value (Utilities|Map|Find (Variables|Default|GetTransforms) _array_element_2))) false))
        (:2
          (Components|InstancedStaticMesh|AddInstances (Variables|Default|GetInner) (.transforms (.Value (Utilities|Map|Find (Variables|Default|GetTransforms) _array_element_2))) false))
        (:3
          (Components|InstancedStaticMesh|AddInstances (Variables|Default|GetEdge) (.transforms (.Value (Utilities|Map|Find (Variables|Default|GetTransforms) _array_element_2))) false))))
    (return)))

(fn GetBitmaskValue
  (params (CurrentPixelX :type Integer) (CurrentPixelY :type Integer))
  (bind _lbitmask (LocalVariables|GetLBitmask))
  (bind _lbitmask_2 (LocalVariables|GetLBitmask))
  (bind _lbitmask_3 (LocalVariables|GetLBitmask))
  (bind _lbitmask_4 (LocalVariables|GetLBitmask))
  (bind _enumvalue (|ForEachEDirection8)
    (:LoopBody
      (switch Utilities|FlowControl|Switch|SwitchonEDirection8 _enumvalue
        (:NewEnumerator0
          (bind (_x _y) (CallFunction|GetTileinDirection _enumvalue (Utilities|Struct|MakeFGridIndex CurrentPixelX CurrentPixelY) :!label _label))
          (if (== (.FoundColor (Class|VictoryBPFunctionLibrary|VictoryGetPixel (Variables|Default|GetPixelArray) (.y (Variables|Default|GetTerrainSize)) _x _y)) "(R=1.000000,G=1.000000,B=1.000000,A=1.000000)")
            (Utilities|Map|Add (LocalVariables|GetLBitmask) _enumvalue 1)))
        (:NewEnumerator1
          (goto _label))
        (:NewEnumerator2
          (goto _label))
        (:NewEnumerator3
          (goto _label))
        (:NewEnumerator4
          (if (or (== (.Value (Utilities|Map|Find _lbitmask_3 "NewEnumerator0")) 1) (== (.Value (Utilities|Map|Find _lbitmask_3 "NewEnumerator1")) 1))
            (goto _label)))
        (:NewEnumerator5
          (if (or (== (.Value (Utilities|Map|Find _lbitmask_4 "NewEnumerator0")) 1) (== (.Value (Utilities|Map|Find _lbitmask_4 "NewEnumerator2")) 1))
            (goto _label)))
        (:NewEnumerator6
          (if (or (== (.Value (Utilities|Map|Find _lbitmask_2 "NewEnumerator3")) 1) (== (.Value (Utilities|Map|Find _lbitmask_2 "NewEnumerator1")) 1))
            (goto _label)))
        (:NewEnumerator7
          (if (or (== (.Value (Utilities|Map|Find _lbitmask "NewEnumerator3")) 1) (== (.Value (Utilities|Map|Find _lbitmask "NewEnumerator2")) 1))
            (goto _label)))))
    (:then
      ;[1 1 1] Calculates bitmask value
      (bind _values (Utilities|Map|Values (LocalVariables|GetLBitmask)))
      (for (_array_element _array_index) _values
        (LocalVariables|SetLBitmaskValue (+ (LocalVariables|GetLBitmaskValue) (* (Math|Float|Truncate (Math|Float|Power 2.0 (Math|Conversions|ToFloat(Integer) _array_index))) _array_element))))
      (return (LocalVariables|GetLBitmaskValue)))))

(fn GetTileinDirection
  (params (Direction :type EDirection8%20Enum :default "NewEnumerator0") (Index :type F%20Grid%20Index%20Structure))
  (switch Utilities|FlowControl|Switch|SwitchonEDirection8 Direction
    (:NewEnumerator0
      (return (.x Index) (+ (.y Index) -1)))
    (:NewEnumerator1
      (return (+ (.x Index) -1) (.y Index)))
    (:NewEnumerator2
      (return (+ (.x Index) 1) (.y Index)))
    (:NewEnumerator3
      (return (.x Index) (+ (.y Index) 1)))
    (:NewEnumerator4
      (return (+ (.x Index) -1) (+ (.y Index) -1)))
    (:NewEnumerator5
      (return (+ (.x Index) 1) (+ (.y Index) -1)))
    (:NewEnumerator6
      (return (+ (.x Index) -1) (+ (.y Index) 1)))
    (:NewEnumerator7
      (return (+ (.x Index) 1) (+ (.y Index) 1)))))