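; BP_EventManager holds a queue of event objects and runs them in order.
; Events are added or removed through QueueEvent and RemoveEventFromQueue, and RunNextEvent runs the head as CurrentEvent without dequeuing it.
; RunAllQueuedEvents runs each valid event, using a latent DelayWhile to wait until it becomes invalid before continuing, then clears the queue.
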(event Custom|RunNextEvent
  (if (> (Utilities|Array|Length (Variables|Default|GetEventQueue)) 0)
    (bind _output_get (Variables|Default|SetCurrentEvent (Utilities|Array|Get(acopy) (Variables|Default|GetEventQueue))))
    (Default|RunEvent _output_get)
    (else
      (Variables|Default|SetCurrentEvent 0))))

(event Custom|QueueEvent
  (params (Event :type BP%20Event%20Object%20Reference))
  (Utilities|Array|Add (Variables|Default|GetEventQueue) Event))

(event Custom|RemoveEventFromQueue
  (params (Event :type BP%20Event%20Object%20Reference))
  (Utilities|Array|RemoveItem (Variables|Default|GetEventQueue) Event))

(event Custom|RunAllQueuedEvents
  (for _array_element (Variables|Default|GetEventQueue)
    (Utilities|IsValid _array_element
      (:Is%20Valid
        (Default|RunEvent _array_element)
        (Utilities|DelayWhile (Utilities|IsValid _array_element)))))
  (Utilities|Array|Clear (Variables|Default|GetEventQueue)))

(fn ConstructionScript)