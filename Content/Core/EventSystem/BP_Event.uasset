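; BP_Event is an event actor for the game's event system that either runs immediately or queues itself with BP_EventManager.
; Its construction script checks the Instant flag, calling RunEvent when set and otherwise QueueEvent, which finds the manager with GetActorOfClass and passes itself in.
; RunEvent is an empty hook for the event's behavior, and EndEvent destroys the actor.
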(event Custom|RunEvent)

(event Custom|EndEvent
  (Actor|DestroyActor))

(event Custom|QueueEvent
  (bind _returnvalue (Actor|GetActorOfClass "/Game/Core/EventSystem/BP_EventManager.BP_EventManager_C"))
  (bind _output_get (Variables|Default|SetEventManagerRef _returnvalue))
  (Default|QueueEvent _output_get self))

(fn ConstructionScript
  (if (Variables|Default|GetbInstant)
    (CallFunction|RunEvent)
    (else
      (CallFunction|QueueEvent))))